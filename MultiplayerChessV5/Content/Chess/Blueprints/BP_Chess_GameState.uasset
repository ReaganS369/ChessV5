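; Game state for a networked chess game that starts play once two players join, manages turns and per-color clocks, and decides game over.
; After each move it tests the next player's king for check and simulates candidate moves until one is safe, yielding checkmate, stalemate or insufficient material.
; Asynchronous piece calculations are awaited through short Delay polling loops.
; Multicast-style events refresh squares and each local pawn's HUD with turn changes or results.
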(event Custom|TurnAccountUp
  ;[1 1 1] Turn Management
  (CallFunction|AnalysetheSituation)
  (if (Variables|system|GetTurnAnalyseReady) :!label _label
    (if (not (Variables|System|GetInsufficientMaterial))
      (if (Variables|System|GetAtLeastOneMoveAvailableForNextPlayer)
        (CallFunction|STurnAccountUp)
        (elif (Variables|System|GetNextPlayerKingIsInCheck)
          (CallFunction|FinishtheGame 1)
          (else
            (CallFunction|FinishtheGame 2))))
      (else
        (CallFunction|FinishtheGame 3)))
    (else
      (Utilities|FlowControl|Delay 0.01)
      (goto _label))))

(event Custom|S_TurnAccountUp
  ;[1 1 1] Turn Management
  (bind _result (Math|Integer|IncrementInt (Variables|system|GetTurnAccount))
    (:%20%20
      (Variables|system|SetTurnAccount _result)
      (if (< (Variables|system|GetColorTurn) (Variables|Default|GetMaxPlayersInGame))
        (bind _result_2 (Math|Integer|IncrementInt (Variables|system|GetColorTurn))
          (:%20%20
            (Variables|system|SetColorTurn _result_2)))
        (else
          (Variables|system|SetColorTurn 1)))
      ;;[1 1 1] Un select square
      (CallFunction|MUpdateSquaresandHUD))))

(event Custom|ClockPorcess
  ;[1 1 1] Clock Management
  (switch int (Variables|system|GetColorTurn)
    (:1
      (if (> (Variables|System|GetWhiteRemainingDecimals) 0.0)
        (Variables|System|SetWhiteRemainingDecimals (- (Variables|System|GetWhiteRemainingDecimals) 0.01))
        (else
          (Variables|System|SetWhiteRemainingDecimals 1.0)
          (switch int (Variables|system|GetColorTurn) :!label _label
            (:1
              (bind _result (Math|Integer|DecrementInt (Variables|System|GetWhiteRemainingTime))
                (:%20%20
                  (bind _output_get (Variables|System|SetWhiteRemainingTime _result))
                  (if (< _output_get 0)
                    (Variables|System|SetWhiteRemainingDecimals 0.0)
                    (Variables|System|SetWhiteRemainingTime 0)
                    (CallFunction|FinishtheGame 5 :!label _label_2)))))
            (:2
              (bind _result_2 (Math|Integer|DecrementInt (Variables|System|GetBlackRemainingTime))
                (:%20%20
                  (bind _output_get_2 (Variables|System|SetBlackRemainingTime _result_2))
                  (if (< _output_get_2 0)
                    (Variables|System|SetBlackRemainingDecimals 0.0)
                    (Variables|System|SetBlackRemainingTime 0)
                    (goto _label_2)))))))))
    (:2
      (if (> (Variables|System|GetBlackRemainingDecimals) 0.0)
        (Variables|System|SetBlackRemainingDecimals (- (Variables|System|GetBlackRemainingDecimals) 0.01))
        (else
          (Variables|System|SetBlackRemainingDecimals 1.0)
          (goto _label))))))

(event Custom|S_GameInit
  (bind _returnvalue (Utilities|Time|SetTimerbyEvent (delegate Custom|IsGameReady) 0.5 true))
  (Variables|System|SetIsGameReadyTimer _returnvalue))

(event Custom|IsGameReady
  (if (> (Utilities|Array|Length (Variables|Default|GetPlayerArray)) 1)
    (Variables|System|SetGameReady true)
    (CallFunction|MRemoveWaitingMessage)
    (CallFunction|ClockStart)
    (Utilities|Time|ClearandInvalidateTimerbyHandle (Variables|System|GetIsGameReadyTimer))))

(event Custom|AnalyseTheSituation
  ;[1 1 1] Analyse Game Situation
  (Variables|system|SetTurnAnalyseReady false)
  (Variables|System|SetNextPlayerKingIsInCheck false)
  (Variables|System|SetAtLeastOneMoveAvailableForNextPlayer false)
  (Variables|System|SetInsufficientMaterial false)
  (Utilities|Array|Clear (Variables|system|GetHostilSquaresForOppositeKing))
  ;;[1 1 1] Get the square under next player king
  (bind _nextplayercolor (CallFunction|GetNextPlayerColor))
  (bind _king (CallFunction|FLGetKing _nextplayercolor))
  (Utilities|IsValid _king
    (:Is%20Valid
      (bind _square (CallFunction|FLGetSquareUnderPiece _king))
      (Utilities|IsValid _square
        (:Is%20Valid
          ;;[1 1 1] Check if opponent King is in Check
          (bind _computedpieces (CallFunction|FLComputeAllOppositeAvailableMoveBeforeKingCheck _nextplayercolor))
          (if (> (Utilities|Array|Length _computedpieces) 0)
            (for _array_element _computedpieces
              (if (Variables|/Game/Chess/Blueprints/ChessPieces/BP_PieceParent.BP_PieceParent_C|GetAvailableMovesBeforeKingCheckReady _array_element) :!label _label
                (Utilities|Array|AppendArray (Variables|system|GetHostilSquaresForOppositeKing) (Variables|/Game/Chess/Blueprints/ChessPieces/BP_PieceParent.BP_PieceParent_C|GetHostilMovesForOppositKing _array_element))
                (else
                  (Utilities|FlowControl|Delay 0.01)
                  (goto _label))))
            (Variables|System|SetNextPlayerKingIsInCheck (Utilities|Array|ContainsItem (Variables|system|GetHostilSquaresForOppositeKing) _square))
            (CallFunction|CheckifGameEnd)
            (else
              (Variables|system|SetTurnAnalyseReady true))))
        (:Is%20Not%20Valid)))
    (:Is%20Not%20Valid
      ;;;[1 1 1] No king in game
      (Variables|system|SetTurnAnalyseReady true))))

(event Custom|CheckIfGameEnd
  ;[1 1 1] Check for Insufficient material situation
  (bind _outactors (Actor|GetAllActorsOfClass "/Game/Chess/Blueprints/ChessPieces/BP_PieceParent.BP_PieceParent_C"))
  (if (> (Utilities|Array|Length _outactors) 2)
    ;[1 1 1] Is it still possible to move for the next player?
    (bind _computedpieces (CallFunction|FLComputeAllOppositeAvailableMoveBeforeKingCheck (Variables|system|GetColorTurn)))
    (bind _array_element (Utilities|Array|ForEachLoopwithBreak _computedpieces :!label _label)
      (:LoopBody
        (Default|GetAvailableMoveAfterKingCheck _array_element)
        (if (Variables|/Game/Chess/Blueprints/ChessPieces/BP_PieceParent.BP_PieceParent_C|GetAivailableMovesAfterKingCheckReady _array_element)
          (Default|GetFinalAvailableMoves _array_element)
          (if (Variables|/Game/Chess/Blueprints/ChessPieces/BP_PieceParent.BP_PieceParent_C|GetFinalAvailableMovesReady _array_element) :!label _label_2
            (Utilities|Array|Clear (Variables|/Game/Chess/Blueprints/ChessPieces/BP_PieceParent.BP_PieceParent_C|GetFinalAvailableMovesAfterSimulation _array_element))
            (for _array_element_2 (Variables|/Game/Chess/Blueprints/ChessPieces/BP_PieceParent.BP_PieceParent_C|GetFinalAvailableMovesBeforeSimulation _array_element)
              (Default|SimulateMove _array_element _array_element_2)
              (if (Variables|/Game/Chess/Blueprints/ChessPieces/BP_PieceParent.BP_PieceParent_C|GetMoveSimulationFinished _array_element) :!label _label_3
                (if (not (Variables|/Game/Chess/Blueprints/ChessPieces/BP_PieceParent.BP_PieceParent_C|GetSimulatedKingInDanger _array_element))
                  (Variables|System|SetAtLeastOneMoveAvailableForNextPlayer true)
                  (goto _label Break))
                (else
                  (Utilities|FlowControl|Delay 0.01)
                  (goto _label_3))))
            (else
              (Utilities|FlowControl|Delay 0.01)
              (goto _label_2)))
          (else
            (Utilities|FlowControl|Delay 0.01))))
      (:Completed
        (Variables|system|SetTurnAnalyseReady true)))
    (else
      (Variables|System|SetInsufficientMaterial true)
      (Variables|system|SetTurnAnalyseReady true))))

(event Custom|ClockStart
  (bind _timing (Variables|Default|GetTiming))
  (bind _returnvalue (* _timing 60))
  ;[1 1 1] Clock Management
  (Variables|System|SetWhiteRemainingTime _returnvalue)
  (Variables|System|SetBlackRemainingTime _returnvalue)
  (bind _returnvalue_2 (Utilities|Time|SetTimerbyEvent (delegate Custom|ClockPorcess) 0.01 true))
  (Variables|System|SetClockTimer _returnvalue_2))

(event Custom|Finish%20the%20Game
  (params (GameOverSituation :type Integer))
  ;[0 0.03547 1] The game is finished
  (Variables|System|SetGameOverSituation GameOverSituation)
  (Variables|System|SetGameFinished true)
  (Utilities|Time|ClearandInvalidateTimerbyHandle (Variables|System|GetClockTimer))
  (CallFunction|MUpdateSquaresandHUD))

(event Custom|M_UpdateSquaresAndHUD
  ;[1 1 1] Un select all squares
  (Variables|/Game/Chess/Blueprints/ChessBoard/BP_ChessBoard.BP_ChessBoard_C|SetSelectedSquare (Variables|system|GetChessBoard) 0)
  (bind _outactors (Actor|GetAllActorsOfClass "/Game/Chess/Blueprints/ChessBoard/BP_Square.BP_Square_C"))
  (for _array_element _outactors
    (Default|UnClicked _array_element))
  (bind _asbp_chess_player_pawn (Utilities|Casting|CastToBP_Chess_PlayerPawn (Game|Player|GetPlayerPawn 0)))
  (Utilities|IsValid (Variables|/Game/Chess/Blueprints/BP_Chess_PlayerPawn.BP_Chess_PlayerPawn_C|GetHUD _asbp_chess_player_pawn)
    (:Is%20Valid
      (if (Variables|System|GetGameFinished)
        (switch int (Variables|System|GetGameOverSituation)
          (:1
            (Default|EndGameHUD _asbp_chess_player_pawn "Check Mat"))
          (:2
            (Default|EndGameHUD _asbp_chess_player_pawn "Stalemate"))
          (:3
            (Default|EndGameHUD _asbp_chess_player_pawn "Stalemate"))
          (:4
            (Default|EndGameHUD _asbp_chess_player_pawn "You win: opponent leaved"))
          (:5
            (if (== (Variables|/Game/Chess/Blueprints/BP_Chess_PlayerPawn.BP_Chess_PlayerPawn_C|GetPlayerColor _asbp_chess_player_pawn) (Variables|system|GetColorTurn))
              (Default|EndGameHUD _asbp_chess_player_pawn "Time out")
              (else
                (Default|EndGameHUD _asbp_chess_player_pawn "You Win: Time out")))))
        (else
          (Default|TurnChange (Variables|/Game/Chess/Blueprints/BP_Chess_PlayerPawn.BP_Chess_PlayerPawn_C|GetHUD _asbp_chess_player_pawn)))))))

(event Custom|S_ColorTurnDefinedByFENcode
  (params (ColorTurn :type Integer))
  ;[1 1 1] FEN Code Turn
  (Variables|system|SetColorTurn ColorTurn)
  (Utilities|FlowControl|Delay 1.0)
  (CallFunction|AnalysetheSituation)
  (if (Variables|system|GetTurnAnalyseReady) :!label _label
    (if (not (Variables|System|GetInsufficientMaterial))
      (if (Variables|System|GetAtLeastOneMoveAvailableForNextPlayer)
        (CallFunction|MUpdateSquaresandHUD)
        (elif (Variables|System|GetNextPlayerKingIsInCheck)
          (CallFunction|FinishtheGame 1)
          (else
            (CallFunction|FinishtheGame 2))))
      (else
        (CallFunction|FinishtheGame 3)))
    (else
      (Utilities|FlowControl|Delay 0.01)
      (goto _label))))

(event Custom|M_RemoveWaitingMessage
  (bind _asbp_chess_player_pawn (Utilities|Casting|CastToBP_Chess_PlayerPawn (Game|Player|GetPlayerPawn 0)))
  (Default|RemoveWaitingMsg (Variables|/Game/Chess/Blueprints/BP_Chess_PlayerPawn.BP_Chess_PlayerPawn_C|GetHUD _asbp_chess_player_pawn)))

(event EventBeginPlay
  (bind _returnvalue (Actor|GetActorOfClass "/Game/Chess/Blueprints/ChessBoard/BP_ChessBoard.BP_ChessBoard_C" :!label _label))
  (Utilities|IsValid _returnvalue
    (:Is%20Valid
      (Variables|system|SetChessBoard _returnvalue)
      (CallFunction|SGameInit))
    (:Is%20Not%20Valid
      (Utilities|FlowControl|Delay 0.2)
      (goto _label))))

(fn ConstructionScript)

(fn OnRepTurnAccount)

(fn OnRepColorTurn)

(fn GetNextPlayerColor
  (if (< (Variables|system|GetColorTurn) (Variables|Default|GetMaxPlayersInGame))
    (return (+ (Variables|system|GetColorTurn) 1))
    (else
      (return 1))))

(fn OnRepGameFinished)

(fn OnRepGameOverSituation)

(fn OnRepWhiteRemainingTime)

(fn OnRepBlackRemainingTime)

(fn OnRepWhiteRemainingDecimals)

(fn OnRepBlackRemainingDecimals)

(fn OnRepGameReady)
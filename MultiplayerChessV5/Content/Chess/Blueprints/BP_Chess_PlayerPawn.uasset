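; Player pawn for a networked chess game, handling piece moves, HUD and clock, end-game widget and camera.
; MovePiece routes pawns through en passant and promotion checks and kings through castling, then updates pieces and GameState's turn count.
; S_, M_ and O_ events split server, multicast and owner steps.
; PlayerColor comes from PlayerArray length, its OnRep flips black's view, and the mouse wheel tilts the camera.
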(event Custom|EndGameHUD
  (params (Message :type Text))
  ;[1 1 1] Game Over
  (bind _returnvalue (UserInterface|CreateWidget "/Game/Chess/Blueprints/HUD/WBP_GameEnd.WBP_GameEnd_C" (Game|GetPlayerController 0)))
  (Utilities|IsValid _returnvalue
    (:Is%20Valid
      (Default|DefineMsg _returnvalue Message)
      (UserInterface|Viewport|AddtoViewport _returnvalue 0))))

(event Custom|S_MovePiece
  (params (TargetedSquare :type BP%20Square%20Object%20Reference) (PieceToMove :type BP%20Piece%20Parent%20Object%20Reference))
  ;[1 1 1] Move a piece - this is controlled by "BP_Square"
  (bind (_pieceonsquare _valid) (CallFunction|FLGetPieceonSquare TargetedSquare))
  (if _valid
    (CallFunction|SDestroyPiece _pieceonsquare))
  (Variables|/Game/Chess/Blueprints/ChessPieces/BP_PieceParent.BP_PieceParent_C|SetCurrentY PieceToMove (Variables|/Game/Chess/Blueprints/ChessBoard/BP_Square.BP_Square_C|GetY TargetedSquare))
  (Variables|/Game/Chess/Blueprints/ChessPieces/BP_PieceParent.BP_PieceParent_C|SetCurrentX PieceToMove (Variables|/Game/Chess/Blueprints/ChessBoard/BP_Square.BP_Square_C|GetX TargetedSquare))
  ;;[1 1 1] Needed for "En passant" take (pawns) and Castling
  (Variables|/Game/Chess/Blueprints/ChessPieces/BP_PieceParent.BP_PieceParent_C|SetTurnWhenLastMove PieceToMove (+ (Variables|/Game/Chess/Blueprints/BP_Chess_GameState.BP_Chess_GameState_C|GetTurnAccount (Variables|Default|GetAs%20GS%20Game%20State)) 1))
  (CallFunction|MMovePiece PieceToMove TargetedSquare)
  (Default|TurnAccountUp (Variables|Default|GetAs%20GS%20Game%20State)))

(event Custom|S_DestroyPiece
  (params (PieceToDestroy :type BP%20Piece%20Parent%20Object%20Reference))
  ;[1 1 1] Move a piece - this is controlled by "BP_Square"
  (Actor|DestroyActor PieceToDestroy))

(event Custom|S_PawnPromotionAction
  (params (ClassToSpawn :type BP%20Piece%20Parent%20Class%20Reference) (TargetedSquare :type BP%20Square%20Object%20Reference) (PieceToMove :type BP%20Piece%20Parent%20Object%20Reference))
  ;[1 1 1] Move a piece - this is controlled by "BP_Square"
  ;;[1 1 1] Pawn specific process
  ;;;[1 1 1] Destroy the piece in the targeted square if needed (to do before spawning a new piece)
  (bind (_pieceonsquare _valid) (CallFunction|FLGetPieceonSquare TargetedSquare))
  (if _valid
    (CallFunction|SDestroyPiece self _pieceonsquare))
  (bind _returnvalue (Game|SpawnActorfromClass ClassToSpawn (Math|Transform|MakeTransform (Transformation|GetActorLocation TargetedSquare) "0, 0, 0" (Transformation|GetActorScale3D PieceToMove)) "Undefined" "MultiplyWithRoot" 0 (Variables|/Game/Chess/Blueprints/ChessPieces/BP_PieceParent.BP_PieceParent_C|GetPieceColor PieceToMove) (Variables|/Game/Chess/Blueprints/ChessBoard/BP_Square.BP_Square_C|GetY TargetedSquare) (Variables|/Game/Chess/Blueprints/ChessBoard/BP_Square.BP_Square_C|GetX TargetedSquare) 0))
  (Utilities|IsValid _returnvalue
    (:Is%20Valid
      (Default|PieceColorInit _returnvalue)
      (CallFunction|SDestroyPiece self PieceToMove)
      (Default|TurnAccountUp (Variables|Default|GetAs%20GS%20Game%20State)))
    (:Is%20Not%20Valid
      (Development|PrintString "WBP_PawnPromotion \"Error: piece to spawn had not been spawned\""))))

(event Custom|PawnPromotionAction
  (params (DesiredPieceClass :type BP%20Piece%20Parent%20Class%20Reference) (TargetedSquare :type BP%20Square%20Object%20Reference) (PieceToMove :type BP%20Piece%20Parent%20Object%20Reference))
  ;[1 1 1] Move a piece - this is controlled by "BP_Square"
  ;;[1 1 1] Pawn specific process
  (CallFunction|SPawnPromotionAction DesiredPieceClass TargetedSquare PieceToMove))

(event Custom|S_CastelingCheck
  (params (TargetedSquare :type BP%20Square%20Object%20Reference) (PieceToMove :type BP%20Piece%20Parent%20Object%20Reference))
  ;[1 1 1] Move a piece - this is controlled by "BP_Square"
  ;;[0 0.7067 1] king casteling
  ;;;[1 1 1] King is moving 2 squares : it is casteling
  (if (> (Math|Integer|Absolute(Integer) (- (Variables|/Game/Chess/Blueprints/ChessBoard/BP_Square.BP_Square_C|GetX TargetedSquare) (Variables|/Game/Chess/Blueprints/ChessPieces/BP_PieceParent.BP_PieceParent_C|GetCurrentX PieceToMove))) 1)
    ;;;[1 1 1] True : small Casteling
    ;;; False : large casteling
    (if (> (Variables|/Game/Chess/Blueprints/ChessBoard/BP_Square.BP_Square_C|GetX TargetedSquare) (Variables|/Game/Chess/Blueprints/ChessPieces/BP_PieceParent.BP_PieceParent_C|GetCurrentX PieceToMove))
      ;;;[1 1 1] Move the rook
      (bind _pieceonsquare (CallFunction|FLGetPieceonSquarebyCoordonnates 8 (Variables|/Game/Chess/Blueprints/ChessPieces/BP_PieceParent.BP_PieceParent_C|GetCurrentY PieceToMove)))
      (Variables|/Game/Chess/Blueprints/ChessPieces/BP_PieceParent.BP_PieceParent_C|SetCurrentY _pieceonsquare (Variables|/Game/Chess/Blueprints/ChessPieces/BP_PieceParent.BP_PieceParent_C|GetCurrentY PieceToMove))
      (Variables|/Game/Chess/Blueprints/ChessPieces/BP_PieceParent.BP_PieceParent_C|SetCurrentX _pieceonsquare 6)
      ;;;;[1 1 1] Needed for "En passant" take (pawns) and Castling
      (Variables|/Game/Chess/Blueprints/ChessPieces/BP_PieceParent.BP_PieceParent_C|SetTurnWhenLastMove _pieceonsquare (+ (Variables|/Game/Chess/Blueprints/BP_Chess_GameState.BP_Chess_GameState_C|GetTurnAccount (Variables|Default|GetAs%20GS%20Game%20State)) 1))
      (bind (_square _exists) (CallFunction|FLGetSquarebyCoordonnate (Variables|/Game/Chess/Blueprints/ChessPieces/BP_PieceParent.BP_PieceParent_C|GetCurrentX _pieceonsquare) (Variables|/Game/Chess/Blueprints/ChessPieces/BP_PieceParent.BP_PieceParent_C|GetCurrentY _pieceonsquare)))
      (if _exists
        (CallFunction|MMovePiece _pieceonsquare _square)
        (CallFunction|SMovePiece TargetedSquare PieceToMove :!label _label))
      (else
        (bind _pieceonsquare_2 (CallFunction|FLGetPieceonSquarebyCoordonnates 1 (Variables|/Game/Chess/Blueprints/ChessPieces/BP_PieceParent.BP_PieceParent_C|GetCurrentY PieceToMove)))
        (Variables|/Game/Chess/Blueprints/ChessPieces/BP_PieceParent.BP_PieceParent_C|SetCurrentY _pieceonsquare_2 (Variables|/Game/Chess/Blueprints/ChessPieces/BP_PieceParent.BP_PieceParent_C|GetCurrentY PieceToMove))
        (Variables|/Game/Chess/Blueprints/ChessPieces/BP_PieceParent.BP_PieceParent_C|SetCurrentX _pieceonsquare_2 4)
        (Variables|/Game/Chess/Blueprints/ChessPieces/BP_PieceParent.BP_PieceParent_C|SetTurnWhenLastMove _pieceonsquare_2 (+ (Variables|/Game/Chess/Blueprints/BP_Chess_GameState.BP_Chess_GameState_C|GetTurnAccount (Variables|Default|GetAs%20GS%20Game%20State)) 1))
        (bind (_square_2 _exists_2) (CallFunction|FLGetSquarebyCoordonnate (Variables|/Game/Chess/Blueprints/ChessPieces/BP_PieceParent.BP_PieceParent_C|GetCurrentX _pieceonsquare_2) (Variables|/Game/Chess/Blueprints/ChessPieces/BP_PieceParent.BP_PieceParent_C|GetCurrentY _pieceonsquare_2)))
        (if _exists_2
          (CallFunction|MMovePiece _pieceonsquare_2 _square_2)
          (goto _label))))
    (else
      (CallFunction|SMovePiece TargetedSquare PieceToMove))))

(event Custom|M_MovePiece
  (params (Piece%20to%20Move :type BP%20Piece%20Parent%20Object%20Reference) (TargetedSquare :type BP%20Square%20Object%20Reference))
  (bind _returnvalue (Transformation|GetActorLocation TargetedSquare))
  ;[1 1 1] Move a piece - this is controlled by "BP_Square"
  (Utilities|IsValid TargetedSquare
    (:Is%20Valid
      (Transformation|SetActorLocation Piece%20to%20Move (Math|Vector|MakeVector (.x _returnvalue) (.y _returnvalue) (.z _returnvalue)) false false))
    (:Is%20Not%20Valid
      (Development|PrintString "Pawn_Player : \"Error : targeted square not found\""))))

(event Custom|MovePiece
  (params (TargetedSquare :type BP%20Square%20Object%20Reference) (PieceToMove :type BP%20Piece%20Parent%20Object%20Reference))
  ;[1 1 1] Move a piece - this is controlled by "BP_Square"
  (Variables|Default|SetTargeted%20Square TargetedSquare)
  (Variables|Default|SetPiece%20to%20Move PieceToMove)
  (if (== (Variables|/Game/Chess/Blueprints/ChessPieces/BP_PieceParent.BP_PieceParent_C|GetPieceType PieceToMove) 1)
    (CallFunction|PawnTakeEnPassantCheck (Variables|Default|GetTargeted%20Square) (Variables|Default|GetPiece%20to%20Move))
    (elif (== (Variables|/Game/Chess/Blueprints/ChessPieces/BP_PieceParent.BP_PieceParent_C|GetPieceType (Variables|Default|GetPiece%20to%20Move)) 6)
      (CallFunction|SCastelingCheck (Variables|Default|GetTargeted%20Square) (Variables|Default|GetPiece%20to%20Move))
      (else
        (CallFunction|SMovePiece (Variables|Default|GetTargeted%20Square) (Variables|Default|GetPiece%20to%20Move))))))

(event Custom|O_CreatePawnPromotionHUD
  (params (TargetedSquare :type BP%20Square%20Object%20Reference) (PieceToMove :type BP%20Piece%20Parent%20Object%20Reference))
  ;[1 1 1] Move a piece - this is controlled by "BP_Square"
  (bind _returnvalue (UserInterface|CreateWidget "/Game/Chess/Blueprints/HUD/WBP_PawnPromotion.WBP_PawnPromotion_C" 0 PieceToMove TargetedSquare self))
  (UserInterface|Viewport|AddtoViewport _returnvalue 0))

(event Custom|ClockUpdate
  ;[1 1 1] Clock update
  (if (Variables|/Game/Chess/Blueprints/BP_Chess_GameState.BP_Chess_GameState_C|GetGameReady (Variables|Default|GetAs%20GS%20Game%20State))
    (Utilities|IsValid (Variables|Default|GetHUD)
      (:Is%20Valid
        (Default|UpdateClock (Variables|Default|GetHUD))))))

(event Custom|InitClockTimer
  ;[1 1 1] Clock update
  (Utilities|Time|SetTimerbyEvent (delegate Custom|ClockUpdate) 0.01 true))

(event Custom|S_PlayerColor
  ;[1 1 1] Give a color to a player
  (Variables|Default|SetPlayerColor (Utilities|Array|Length (Variables|/Script/Engine.GameStateBase|GetPlayerArray (Variables|Default|GetAs%20GS%20Game%20State)))))

(event Custom|HUDInit
  ;[1 1 1] Move a piece - this is controlled by "BP_Square"
  (if (Pawn|IsLocallyControlled)
    (bind _returnvalue (UserInterface|CreateWidget "/Game/Chess/Blueprints/HUD/WBP_HUD.WBP_HUD_C"))
    (Utilities|IsValid _returnvalue
      (:Is%20Valid
        (Variables|Default|SetHUD _returnvalue)
        (UserInterface|Viewport|AddtoViewport _returnvalue 0)))))

(event Custom|CheckForPawnPromotion
  (params (TargetedSquare :type BP%20Square%20Object%20Reference) (PieceToMove :type BP%20Piece%20Parent%20Object%20Reference))
  ;[1 1 1] Move a piece - this is controlled by "BP_Square"
  ;;[1 1 1] Pawn Promotion Check
  (if (== (Variables|/Game/Chess/Blueprints/ChessPieces/BP_PieceParent.BP_PieceParent_C|GetPieceType PieceToMove) 1)
    (switch int (Variables|/Game/Chess/Blueprints/ChessPieces/BP_PieceParent.BP_PieceParent_C|GetPieceColor PieceToMove)
      (:Default
        (CallFunction|SMovePiece TargetedSquare PieceToMove :!label _label))
      (:1
        (if (== (Variables|/Game/Chess/Blueprints/ChessBoard/BP_Square.BP_Square_C|GetY TargetedSquare) (Variables|/Game/Chess/Blueprints/ChessBoard/BP_ChessBoard.BP_ChessBoard_C|GetMaxY (Variables|Default|GetChessBoard)))
          (CallFunction|SCreatePawnPromotionHUD TargetedSquare PieceToMove :!label _label_2)
          (else
            (goto _label))))
      (:2
        (if (== (Variables|/Game/Chess/Blueprints/ChessBoard/BP_Square.BP_Square_C|GetY TargetedSquare) 1)
          (goto _label_2)
          (else
            (goto _label)))))
    (else
      (goto _label))))

(event Custom|CamAdjustment
  ;[1 1 1] Called from OnRep_PlayerColor
  ;[1 1 1] Adjust the cam for black player
  (Utilities|FlowControl|Delay 0.2)
  (if (Pawn|IsLocallyControlled)
    (if (== (Variables|Default|GetPlayerColor) 2)
      (Transformation|SetActorTransform (Math|Transform|MakeTransform (Math|Vector|MakeVector 6e+02 4e+02 4e+02) "0.000000,180.000000,0.000000" "1.000000,1.000000,1.000000")))))

(event Custom|S_CreatePawnPromotionHUD
  (params (TargetedSquare :type BP%20Square%20Object%20Reference) (PieceToMove :type BP%20Piece%20Parent%20Object%20Reference))
  ;[1 1 1] Move a piece - this is controlled by "BP_Square"
  (CallFunction|OCreatePawnPromotionHUD TargetedSquare PieceToMove))

(event Custom|PawnTakeEnPassantCheck
  (params (TargetedSquare :type BP%20Square%20Object%20Reference) (PieceToMove :type BP%20Piece%20Parent%20Object%20Reference))
  (bind _currentx (Variables|/Game/Chess/Blueprints/ChessPieces/BP_PieceParent.BP_PieceParent_C|GetCurrentX PieceToMove))
  (bind _x (Variables|/Game/Chess/Blueprints/ChessBoard/BP_Square.BP_Square_C|GetX TargetedSquare))
  (bind _returnvalue (!= _x _currentx))
  ;[1 1 1] Move a piece - this is controlled by "BP_Square"
  ;;[1 1 1] Pawn specific process
  ;;;[1 1 1] "En passant" check
  (if (== (Variables|/Game/Chess/Blueprints/ChessPieces/BP_PieceParent.BP_PieceParent_C|GetPieceType PieceToMove) 1)
    (bind _valid (CallFunction|FLGetPieceonSquare TargetedSquare))
    (if _valid
      (CallFunction|CheckforPawnPromotion TargetedSquare PieceToMove :!label _label)
      (else
        (switch int (Variables|/Game/Chess/Blueprints/ChessPieces/BP_PieceParent.BP_PieceParent_C|GetPieceColor PieceToMove)
          (:Default
            (goto _label))
          (:1
            (if (== (Variables|/Game/Chess/Blueprints/ChessPieces/BP_PieceParent.BP_PieceParent_C|GetCurrentY PieceToMove) 5)
              ;;;[1 1 1] If True : A pawn is processing a diagonal move on an empty square : it's a take "en passant"
              (if _returnvalue
                (bind _pieceonsquare (CallFunction|FLGetPieceonSquarebyCoordonnates (Variables|/Game/Chess/Blueprints/ChessBoard/BP_Square.BP_Square_C|GetX TargetedSquare) (+ (Variables|/Game/Chess/Blueprints/ChessBoard/BP_Square.BP_Square_C|GetY TargetedSquare) -1)))
                (CallFunction|SDestroyPiece _pieceonsquare))
              (else
                (goto _label))))
          (:2
            (if (== (Variables|/Game/Chess/Blueprints/ChessPieces/BP_PieceParent.BP_PieceParent_C|GetCurrentY PieceToMove) 4)
              (if _returnvalue
                (bind _pieceonsquare_2 (CallFunction|FLGetPieceonSquarebyCoordonnates (Variables|/Game/Chess/Blueprints/ChessBoard/BP_Square.BP_Square_C|GetX TargetedSquare) (+ (Variables|/Game/Chess/Blueprints/ChessBoard/BP_Square.BP_Square_C|GetY TargetedSquare) 1)))
                (CallFunction|SDestroyPiece _pieceonsquare_2))
              (else
                (goto _label)))))
        (CallFunction|SMovePiece TargetedSquare PieceToMove)))
    (else
      (goto _label))))

(event EventBeginPlay
  (Utilities|FlowControl|Sequence
    (:then_0
      (CallFunction|HUDInit))
    (:then_1
      (bind _asgs_game_state (Utilities|Casting|CastToBP_Chess_GameState (Game|GetGameState) :!label _label)
        (:then
          (Variables|Default|SetAs%20GS%20Game%20State _asgs_game_state)
          (CallFunction|SPlayerColor)
          (CallFunction|InitClockTimer))
        (:CastFailed
          (Utilities|FlowControl|Delay 0.2)
          (Development|PrintString "Pawn_Player : \"GameState Not Found\"")
          (goto _label))))
    (:then_2
      (Transformation|SetActorTransform (Math|Transform|MakeTransform (Math|Vector|MakeVector 3e+02 4e+02 4e+02) "0, 0, 0" "1.000000,1.000000,1.000000")))
    (:then_3
      (bind _returnvalue (Actor|GetActorOfClass "/Game/Chess/Blueprints/ChessBoard/BP_ChessBoard.BP_ChessBoard_C"))
      (Variables|Default|SetChessBoard _returnvalue))))

(event Input|MouseEvents|MouseWheelUp
  (params (Key :type Key%20Structure :default "None"))
  ;[1 1 1] Cam Pitch Control
  (:Pressed
    (if (> (Math|Float|Absolute(Float) (.pitch (Variables|/Script/Engine.SceneComponent|GetRelativeRotation (Variables|Default|GetSpringArm)))) 45.0)
      (Transformation|AddRelativeRotation (Variables|Default|GetSpringArm) (Math|Rotator|MakeRotator 0.0 1.0 0.0) false false)
      (if (== (Variables|Default|GetPlayerColor) 1)
        (Transformation|AddActorWorldOffset self (Math|Vector|MakeVector -1e+01 0.0 0.0))
        (else
          (Transformation|AddActorWorldOffset self (Math|Vector|MakeVector 1e+01 0.0 0.0)))))))

(event Input|MouseEvents|MouseWheelDown
  (params (Key :type Key%20Structure :default "None"))
  ;[1 1 1] Cam Pitch Control
  (:Pressed
    (if (< (Math|Float|Absolute(Float) (.pitch (Variables|/Script/Engine.SceneComponent|GetRelativeRotation (Variables|Default|GetSpringArm)))) 85.0)
      (Transformation|AddRelativeRotation (Variables|Default|GetSpringArm) (Math|Rotator|MakeRotator 0.0 -1.0 0.0) false false)
      (if (== (Variables|Default|GetPlayerColor) 1)
        (Transformation|AddActorWorldOffset self (Math|Vector|MakeVector 1e+01 0.0 0.0))
        (else
          (Transformation|AddActorWorldOffset self (Math|Vector|MakeVector -1e+01 0.0 0.0)))))))

(fn ConstructionScript)

(fn CamInit)

(fn OnRepPlayerColor
  (CallFunction|CamAdjustment))

(fn FIsKinginDanger
  (params (Color :type Integer)))
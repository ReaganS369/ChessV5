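; Chess board actor that builds the square grid and spawns the starting pieces.
; On BeginPlay it waits for the chess game state, then takes a layout from the game instance's FEN code or from preset/test arrays.
; The FEN parser sets the side to move and fills a spawn list, which grid generation reads while skipping configured holes.
; FEN castling rights become prevention flags on kings; a separate piece-spawning event is unused.
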(event Custom|FenConvertor
  (params (FENString :type String))
  (bind _as_gs_game_state (Variables|System|GetAs%20GS%20Game%20State))
  ;[1 1 1] FEN Interpreter
  (Variables|FenEncode|SetFENString FENString)
  (if (Utilities|String|Contains FENString "w" false true)
    (Default|SColorTurnDefinedbyFENcode _as_gs_game_state 1)
    (else
      (Default|SColorTurnDefinedbyFENcode _as_gs_game_state 2)))
  (Variables|FenEncode|SetCurrentFenCharacter "")
  (Variables|FenEncode|SetFENLocX 1)
  (Variables|FenEncode|SetFENLocY (Variables|Settings|GetMaxY))
  (Utilities|Array|Clear (Variables|FenEncode|GetFenEncode))
  (bind _array_element (Utilities|Array|ForEachLoopwithBreak (Utilities|String|GetCharacterArrayfromString (Variables|FenEncode|GetFENString)) :!label _label)
    (:LoopBody
      (Variables|FenEncode|SetCurrentFenCharacter _array_element)
      (switch string _array_element
        (:Default
          (if (Class|KismetStringLibrary|IsNumeric (Variables|FenEncode|GetCurrentFenCharacter))
            (Variables|FenEncode|SetFENLocX (+ (Variables|FenEncode|GetFENLocX) (Math|Conversions|ToInteger(Byte) (Variables|FenEncode|GetCurrentFenCharacter))))
            (else
              (goto _label Break))))
        (:None
          (goto _label Break))
        (:/
          (Variables|FenEncode|SetFENLocY (+ (Variables|FenEncode|GetFENLocY) -1))
          (Variables|FenEncode|SetFENLocX 1))
        (:r
          (Variables|FenEncode|SetFENCurrentPieceType 4)
          (Variables|FenEncode|SetFENCurrentColor 2)
          (Utilities|Array|Add (Variables|FenEncode|GetFenEncode) (Utilities|Struct|MakeStruct_SpawningEncode (Variables|FenEncode|GetFENCurrentColor) (Variables|FenEncode|GetFENCurrentPieceType) (Variables|FenEncode|GetFENLocX) (Variables|FenEncode|GetFENLocY)) :!label _label_2)
          (Variables|FenEncode|SetFENLocX (+ (Variables|FenEncode|GetFENLocX) 1)))
        (:n
          (Variables|FenEncode|SetFENCurrentPieceType 2)
          (Variables|FenEncode|SetFENCurrentColor 2)
          (goto _label_2))
        (:b
          (Variables|FenEncode|SetFENCurrentPieceType 3)
          (Variables|FenEncode|SetFENCurrentColor 2)
          (goto _label_2))
        (:q
          (Variables|FenEncode|SetFENCurrentPieceType 5)
          (Variables|FenEncode|SetFENCurrentColor 2)
          (goto _label_2))
        (:k
          (Variables|FenEncode|SetFENCurrentPieceType 6)
          (Variables|FenEncode|SetFENCurrentColor 2)
          (goto _label_2))
        (:p
          (Variables|FenEncode|SetFENCurrentPieceType 1)
          (Variables|FenEncode|SetFENCurrentColor 2)
          (goto _label_2))
        (:R
          (Variables|FenEncode|SetFENCurrentPieceType 4)
          (Variables|FenEncode|SetFENCurrentColor 1)
          (goto _label_2))
        (:N
          (Variables|FenEncode|SetFENCurrentPieceType 2)
          (Variables|FenEncode|SetFENCurrentColor 1)
          (goto _label_2))
        (:B
          (Variables|FenEncode|SetFENCurrentPieceType 3)
          (Variables|FenEncode|SetFENCurrentColor 1)
          (goto _label_2))
        (:Q
          (Variables|FenEncode|SetFENCurrentPieceType 5)
          (Variables|FenEncode|SetFENCurrentColor 1)
          (goto _label_2))
        (:K
          (Variables|FenEncode|SetFENCurrentPieceType 6)
          (Variables|FenEncode|SetFENCurrentColor 1)
          (goto _label_2))
        (:P
          (Variables|FenEncode|SetFENCurrentPieceType 1)
          (Variables|FenEncode|SetFENCurrentColor 1)
          (goto _label_2))))
    (:Completed
      (CallFunction|SSpawnChessBoardandPieces))))

(event Custom|S_SpawnPieces
  (bind _piecescale (Variables|Settings|GetPieceScale))
  ;[1 1 1] Pieces Spawning - THIS NODE IS NOT USED
  ;;[1 1 1] Not used - you can use it but you will need a delay
  (Utilities|FlowControl|Delay 0.5)
  (Variables|System|SetBP_Square 0)
  (for _array_element (Variables|Spawning|GetClassicChess)
    (bind (_square _exists) (CallFunction|FLGetSquarebyCoordonnate (.X (Utilities|Struct|BreakStruct_SpawningEncode _array_element)) (.Y (Utilities|Struct|BreakStruct_SpawningEncode _array_element))))
    (if _exists
      (Variables|System|SetBP_Square _square)
      ;;[1 1 1] 1 - Pawn
      ;; 2 - Knight
      ;; 3 - Bishop
      ;; 4 - Rook
      ;; 5 - Queen
      ;; 6 - King
      (switch int (.PieceType (Utilities|Struct|BreakStruct_SpawningEncode _array_element))
        (:1
          (Variables|System|SetPieceClass "/Game/Chess/Blueprints/ChessPieces/BP_Piece_Child_Pawn.BP_Piece_Child_Pawn_C"))
        (:2
          (Variables|System|SetPieceClass "/Game/Chess/Blueprints/ChessPieces/BP_Piece_Child_Knight.BP_Piece_Child_Knight_C"))
        (:3
          (Variables|System|SetPieceClass "/Game/Chess/Blueprints/ChessPieces/BP_Piece_Child_Bishop.BP_Piece_Child_Bishop_C"))
        (:4
          (Variables|System|SetPieceClass "/Game/Chess/Blueprints/ChessPieces/BP_Piece_Child_Rook.BP_Piece_Child_Rook_C"))
        (:5
          (Variables|System|SetPieceClass "/Game/Chess/Blueprints/ChessPieces/BP_Piece_Child_Queen.BP_Piece_Child_Queen_C"))
        (:6
          (Variables|System|SetPieceClass "/Game/Chess/Blueprints/ChessPieces/BP_Piece_Child_king.BP_Piece_Child_king_C")))
      (bind _returnvalue (Game|SpawnActorfromClass (Variables|System|GetPieceClass) (Math|Transform|MakeTransform (Math|Vector|MakeVector (.x (Transformation|GetActorLocation (Variables|System|GetBP_Square))) (.y (Transformation|GetActorLocation (Variables|System|GetBP_Square))) (.z (Transformation|GetActorLocation (Variables|System|GetBP_Square)))) (Math|Rotator|MakeRotator 0.0 0.0 0.0) (Math|Vector|MakeVector _piecescale _piecescale _piecescale)) "Undefined" "MultiplyWithRoot" 0 0))
      (bind _asbp_piece_parent (Utilities|Casting|CastToBP_PieceParent _returnvalue))
      (Variables|System|SetAs%20BP%20Piece%20Parent _asbp_piece_parent)
      (Variables|/Game/Chess/Blueprints/ChessPieces/BP_PieceParent.BP_PieceParent_C|SetPieceColor (Variables|System|GetAs%20BP%20Piece%20Parent) (.Color (Utilities|Struct|BreakStruct_SpawningEncode _array_element)))
      (Variables|/Game/Chess/Blueprints/ChessPieces/BP_PieceParent.BP_PieceParent_C|SetCurrentY (Variables|System|GetAs%20BP%20Piece%20Parent) (Variables|/Game/Chess/Blueprints/ChessBoard/BP_Square.BP_Square_C|GetY (Variables|System|GetBP_Square)))
      (Variables|/Game/Chess/Blueprints/ChessPieces/BP_PieceParent.BP_PieceParent_C|SetCurrentX (Variables|System|GetAs%20BP%20Piece%20Parent) (Variables|/Game/Chess/Blueprints/ChessBoard/BP_Square.BP_Square_C|GetX (Variables|System|GetBP_Square)))
      (Default|PieceColorInit (Variables|System|GetAs%20BP%20Piece%20Parent))
      (else
        (Development|PrintString "Hello")))))

(event Custom|S_Spawn_ChessBoardAndPieces
  (bind _piecescale (Variables|Settings|GetPieceScale))
  ;[1 1 1] ChessBoard generation
  (for _index (range 0 (- (Variables|Settings|GetMaxX) 1))
    (Variables|System|SetXIndex _index)
    (for _index_2 (range 0 (- (Variables|Settings|GetMaxY) 1))
      ;;[0 0.4164 1] NEW Feature : This allow you to create holes in your chess board : just fill the "HolesArray" variable with some squares coordonnates and check the result (example: try to fill a square with x=2 y = 2)
      (Variables|System|SetCanSpawnSquare true)
      (bind _array_element (Utilities|Array|ForEachLoopwithBreak (Variables|Spawning|GetHolesArray) :!label _label)
        (:LoopBody
          (if (and (== (.X (Utilities|Struct|BreakStruct_HolesSquares _array_element)) (+ (Variables|System|GetXIndex) 1)) (== (.Y (Utilities|Struct|BreakStruct_HolesSquares _array_element)) (+ _index_2 1)))
            (Variables|System|SetCanSpawnSquare false)
            (goto _label Break)))
        (:Completed
          (if (Variables|System|GetCanSpawnSquare)
            (bind _returnvalue (Game|SpawnActorfromClass "/Game/Chess/Blueprints/ChessBoard/BP_Square.BP_Square_C" (Math|Transform|MakeTransform (+ (Variables|System|GetInitLocation) "100.000000,0.000000,0.000000")) "Undefined" "MultiplyWithRoot" 0 (+ (Variables|System|GetXIndex) 1) (+ _index_2 1) self 0))
            (Variables|System|SetBP_Square _returnvalue)
            (Variables|System|SetInitLocation (+ (Variables|System|GetInitLocation) "100.000000,0.000000,0.000000"))
            ;[1 1 1] Pieces Spawning
            (for _array_element_2 (Variables|FenEncode|GetFenEncode)
              (if (and (== (.X (Utilities|Struct|BreakStruct_SpawningEncode _array_element_2)) (Variables|/Game/Chess/Blueprints/ChessBoard/BP_Square.BP_Square_C|GetX (Variables|System|GetBP_Square))) (== (.Y (Utilities|Struct|BreakStruct_SpawningEncode _array_element_2)) (Variables|/Game/Chess/Blueprints/ChessBoard/BP_Square.BP_Square_C|GetY (Variables|System|GetBP_Square))))
                ;;[1 1 1] 1 - Pawn
                ;; 2 - Knight
                ;; 3 - Bishop
                ;; 4 - Rook
                ;; 5 - Queen
                ;; 6 - King
                (switch int (.PieceType (Utilities|Struct|BreakStruct_SpawningEncode _array_element_2))
                  (:1
                    (Variables|System|SetPieceClass "/Game/Chess/Blueprints/ChessPieces/BP_Piece_Child_Pawn.BP_Piece_Child_Pawn_C"))
                  (:2
                    (Variables|System|SetPieceClass "/Game/Chess/Blueprints/ChessPieces/BP_Piece_Child_Knight.BP_Piece_Child_Knight_C"))
                  (:3
                    (Variables|System|SetPieceClass "/Game/Chess/Blueprints/ChessPieces/BP_Piece_Child_Bishop.BP_Piece_Child_Bishop_C"))
                  (:4
                    (Variables|System|SetPieceClass "/Game/Chess/Blueprints/ChessPieces/BP_Piece_Child_Rook.BP_Piece_Child_Rook_C"))
                  (:5
                    (Variables|System|SetPieceClass "/Game/Chess/Blueprints/ChessPieces/BP_Piece_Child_Queen.BP_Piece_Child_Queen_C"))
                  (:6
                    (Variables|System|SetPieceClass "/Game/Chess/Blueprints/ChessPieces/BP_Piece_Child_king.BP_Piece_Child_king_C")))
                (bind _returnvalue_2 (Game|SpawnActorfromClass (Variables|System|GetPieceClass) (Math|Transform|MakeTransform (Math|Vector|MakeVector (.x (Variables|System|GetInitLocation)) (.y (Variables|System|GetInitLocation)) (+ (.z (Variables|System|GetInitLocation)) 0.0)) (Math|Rotator|MakeRotator 0.0 0.0 0.0) (Math|Vector|MakeVector _piecescale _piecescale _piecescale)) "Undefined" "MultiplyWithRoot" 0 0))
                (bind _asbp_piece_parent (Utilities|Casting|CastToBP_PieceParent _returnvalue_2))
                (Variables|System|SetAs%20BP%20Piece%20Parent _asbp_piece_parent)
                (Variables|/Game/Chess/Blueprints/ChessPieces/BP_PieceParent.BP_PieceParent_C|SetPieceColor (Variables|System|GetAs%20BP%20Piece%20Parent) (.Color (Utilities|Struct|BreakStruct_SpawningEncode _array_element_2)))
                (Variables|/Game/Chess/Blueprints/ChessPieces/BP_PieceParent.BP_PieceParent_C|SetCurrentY (Variables|System|GetAs%20BP%20Piece%20Parent) (Variables|/Game/Chess/Blueprints/ChessBoard/BP_Square.BP_Square_C|GetY (Variables|System|GetBP_Square)))
                (Variables|/Game/Chess/Blueprints/ChessPieces/BP_PieceParent.BP_PieceParent_C|SetCurrentX (Variables|System|GetAs%20BP%20Piece%20Parent) (Variables|/Game/Chess/Blueprints/ChessBoard/BP_Square.BP_Square_C|GetX (Variables|System|GetBP_Square)))
                (Default|PieceColorInit (Variables|System|GetAs%20BP%20Piece%20Parent))))
            (CallFunction|SCheckFENCasteling)
            (else
              (Variables|System|SetInitLocation (+ (Variables|System|GetInitLocation) "100.000000,0.000000,0.000000")))))))
    (Variables|System|SetInitLocation (Math|Vector|MakeVector 0.0 (Math|Conversions|ToFloat(Integer) (* (+ (Variables|System|GetXIndex) 1) (Variables|Settings|GetScaleIncrementation))) 0.0))))

(event Custom|S_CheckFENCasteling
  ;[1 1 1] FEN Interpreter
  (if (not (Utilities|Array|IsEmpty (Variables|FenEncode|GetFENString)))
    (bind _outactors (Actor|GetAllActorsOfClass "/Game/Chess/Blueprints/ChessPieces/BP_Piece_Child_king.BP_Piece_Child_king_C"))
    (if (Utilities|Array|IsNotEmpty _outactors)
      (Variables|FenEncode|SetKings _outactors)
      (if (Utilities|String|Contains (.RightS (Utilities|String|Split (Variables|FenEncode|GetFENString) " ")) "k" true)
        (if (Utilities|String|Contains (.RightS (Utilities|String|Split (Variables|FenEncode|GetFENString) " ")) "q" true) :!label _label
          (if (Utilities|String|Contains (.RightS (Utilities|String|Split (Variables|FenEncode|GetFENString) " ")) "K" true) :!label _label_2
            (if (not (Utilities|String|Contains (.RightS (Utilities|String|Split (Variables|FenEncode|GetFENString) " ")) "Q" true)) :!label _label_3
              (bind _array_element (Utilities|Array|ForEachLoopwithBreak (Variables|FenEncode|GetKings) :!label _label_4)
                (:LoopBody
                  (if (== (Variables|/Game/Chess/Blueprints/ChessPieces/BP_PieceParent.BP_PieceParent_C|GetPieceColor _array_element) 1)
                    (Variables|/Game/Chess/Blueprints/ChessPieces/BP_Piece_Child_king.BP_Piece_Child_king_C|SetLargeCastlePreventedByFEN _array_element true)
                    (goto _label_4 Break)))
                (:Completed)))
            (else
              (bind _array_element_2 (Utilities|Array|ForEachLoopwithBreak (Variables|FenEncode|GetKings) :!label _label_5)
                (:LoopBody
                  (if (== (Variables|/Game/Chess/Blueprints/ChessPieces/BP_PieceParent.BP_PieceParent_C|GetPieceColor _array_element_2) 1)
                    (Variables|/Game/Chess/Blueprints/ChessPieces/BP_Piece_Child_king.BP_Piece_Child_king_C|SetSmallCastlePreventedByFEN _array_element_2 true)
                    (goto _label_5 Break)))
                (:Completed
                  (goto _label_3)))))
          (else
            (bind _array_element_3 (Utilities|Array|ForEachLoopwithBreak (Variables|FenEncode|GetKings) :!label _label_6)
              (:LoopBody
                (if (== (Variables|/Game/Chess/Blueprints/ChessPieces/BP_PieceParent.BP_PieceParent_C|GetPieceColor _array_element_3) 2)
                  (Variables|/Game/Chess/Blueprints/ChessPieces/BP_Piece_Child_king.BP_Piece_Child_king_C|SetLargeCastlePreventedByFEN _array_element_3 true)
                  (goto _label_6 Break)))
              (:Completed
                (goto _label_2)))))
        (else
          (bind _array_element_4 (Utilities|Array|ForEachLoopwithBreak (Variables|FenEncode|GetKings) :!label _label_7)
            (:LoopBody
              (if (== (Variables|/Game/Chess/Blueprints/ChessPieces/BP_PieceParent.BP_PieceParent_C|GetPieceColor _array_element_4) 2)
                (Variables|/Game/Chess/Blueprints/ChessPieces/BP_Piece_Child_king.BP_Piece_Child_king_C|SetSmallCastlePreventedByFEN _array_element_4 true)
                (goto _label_7 Break)))
            (:Completed
              (goto _label))))))))

(event EventBeginPlay
  (bind _testspawningencode (Variables|Spawning|GetTestSpawningEncode))
  (bind _asbp_chess_game_state (Utilities|Casting|CastToBP_Chess_GameState (Game|GetGameState) :!label _label)
    (:then
      (Variables|System|SetAs%20GS%20Game%20State _asbp_chess_game_state)
      (if (Variables|Settings|GetUseFENCode)
        (bind _asbp_gi_chess_game_instance (Utilities|Casting|CastToBP_GI_ChessGameInstance (Game|GetGameInstance)))
        (if (Utilities|Array|IsEmpty (Variables|/Game/Chess/Blueprints/BP_GI_ChessGameInstance.BP_GI_ChessGameInstance_C|GetFENCode _asbp_gi_chess_game_instance))
          (CallFunction|FenConvertor "rnbqkbnr/pppppppp/8/8/8/8/PPPPPPPP/RNBQKBNR w KQkq - 0 1")
          (else
            (CallFunction|FenConvertor (Variables|/Game/Chess/Blueprints/BP_GI_ChessGameInstance.BP_GI_ChessGameInstance_C|GetFENCode _asbp_gi_chess_game_instance))))
        (else
          (if (Utilities|Array|IsEmpty _testspawningencode)
            (Variables|FenEncode|SetFenEncode (Variables|Spawning|GetClassicChess))
            (else
              (Variables|FenEncode|SetFenEncode _testspawningencode)))
          (CallFunction|SSpawnChessBoardandPieces))))
    (:CastFailed
      (Utilities|FlowControl|Delay 0.1)
      (goto _label))))

(fn ConstructionScript)

(fn OnRepBPSquare)

(fn OnRepXIndex)

(fn OnRepasBPPieceParent)
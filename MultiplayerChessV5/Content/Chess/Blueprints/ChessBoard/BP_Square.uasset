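; BP_Square is one chessboard tile: it sets its checker material from X/Y and handles hover, selection and legal-move highlighting on the local player's turn.
; Clicking an own piece runs its staged move computation, polling ready flags with short delays and simulating each move to reject those endangering the king.
; Clicking another square asks the player pawn to move the selected piece if that square is among its filtered moves.
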(event OnBeginCursorOver(Plane)
  (params (TouchedComponent :type Primitive%20Component%20Object%20Reference))
  (bind _as_gs_game_state (Variables|Default|GetAs%20GS%20Game%20State))
  ;[1 1 1] Highlight system
  (Utilities|IsValid _as_gs_game_state
    (:Is%20Valid
      (if (and (not (Variables|/Game/Chess/Blueprints/BP_Chess_GameState.BP_Chess_GameState_C|GetGameFinished _as_gs_game_state)) (Variables|/Game/Chess/Blueprints/BP_Chess_GameState.BP_Chess_GameState_C|GetGameReady _as_gs_game_state))
        (Utilities|MyTurn
          (:Yes
            (if (Variables|Default|GetGameReady)
              (Rendering|Material|SetMaterial (Variables|Default|GetPlane) 0 "/Game/Chess/Materials/MI_HighLighted_MouseOver_Inst.MI_HighLighted_MouseOver_Inst"))))))))

(event OnEndCursorOver(Plane)
  (params (TouchedComponent :type Primitive%20Component%20Object%20Reference))
  ;[1 1 1] Highlight system
  (if (not (Variables|Default|GetClicked))
    (if (Variables|Default|GetAvailableHightLight)
      (CallFunction|HighlightAvailableMoves)
      (elif (Variables|Default|GetGameReady)
        (Rendering|Material|SetMaterial (Variables|Default|GetPlane) 0 (Variables|Default|GetMaterialInit))))))

(event OnClicked(Plane)
  (params (TouchedComponent :type Primitive%20Component%20Object%20Reference) (ButtonPressed :type Key%20Structure :default "None"))
  (bind _chessboard (Variables|Default|GetChessBoard))
  (bind _chessboard_2 (Variables|Default|GetChessBoard))
  (bind _as_gs_game_state (Variables|Default|GetAs%20GS%20Game%20State))
  ;[1 1 1] Selection System "OnClick"
  (Utilities|IsValid _as_gs_game_state
    (:Is%20Valid
      (if (and (not (Variables|/Game/Chess/Blueprints/BP_Chess_GameState.BP_Chess_GameState_C|GetGameFinished _as_gs_game_state)) (Variables|/Game/Chess/Blueprints/BP_Chess_GameState.BP_Chess_GameState_C|GetGameReady _as_gs_game_state))
        (Utilities|MyTurn
          (:Yes
            (bind _playercolor (CallFunction|FLGetPlayerColor))
            ;[1 1 1] Get the piece that is on the square
            (bind (_pieceonsquare _valid) (CallFunction|FLGetPieceonSquare self))
            (if _valid
              (if (== (Variables|/Game/Chess/Blueprints/ChessPieces/BP_PieceParent.BP_PieceParent_C|GetPieceColor _pieceonsquare) _playercolor)
                (Variables|Default|SetClicked true)
                (Variables|/Game/Chess/Blueprints/ChessPieces/BP_PieceParent.BP_PieceParent_C|SetFinalMovesAfterSimulationReady _pieceonsquare false)
                (Utilities|IsValid _chessboard_2
                  (:Is%20Valid
                    (Variables|/Game/Chess/Blueprints/ChessBoard/BP_ChessBoard.BP_ChessBoard_C|SetSelectedSquare _chessboard_2 self)
                    (CallFunction|UnSelectOtherSquares)
                    ;[1 1 1] Available moves highlitghting system
                    ;;[1 1 1] Waiting for event to compute
                    (Default|GetAvailableMoves _pieceonsquare)
                    (if (Variables|/Game/Chess/Blueprints/ChessPieces/BP_PieceParent.BP_PieceParent_C|GetAvailableMovesBeforeKingCheckReady _pieceonsquare) :!label _label
                      (Default|GetAvailableMoveAfterKingCheck _pieceonsquare)
                      (if (Variables|/Game/Chess/Blueprints/ChessPieces/BP_PieceParent.BP_PieceParent_C|GetAivailableMovesAfterKingCheckReady _pieceonsquare) :!label _label_2
                        (Default|GetFinalAvailableMoves _pieceonsquare)
                        (if (Variables|/Game/Chess/Blueprints/ChessPieces/BP_PieceParent.BP_PieceParent_C|GetFinalAvailableMovesReady _pieceonsquare) :!label _label_3
                          (Utilities|Array|Clear (Variables|/Game/Chess/Blueprints/ChessPieces/BP_PieceParent.BP_PieceParent_C|GetFinalAvailableMovesAfterSimulation _pieceonsquare))
                          (for _array_element (Variables|/Game/Chess/Blueprints/ChessPieces/BP_PieceParent.BP_PieceParent_C|GetFinalAvailableMovesBeforeSimulation _pieceonsquare)
                            (Default|SimulateMove _pieceonsquare _array_element)
                            (if (Variables|/Game/Chess/Blueprints/ChessPieces/BP_PieceParent.BP_PieceParent_C|GetMoveSimulationFinished _pieceonsquare) :!label _label_4
                              (if (not (Variables|/Game/Chess/Blueprints/ChessPieces/BP_PieceParent.BP_PieceParent_C|GetSimulatedKingInDanger _pieceonsquare))
                                (Utilities|Array|Add (Variables|/Game/Chess/Blueprints/ChessPieces/BP_PieceParent.BP_PieceParent_C|GetFinalAvailableMovesAfterSimulation _pieceonsquare) _array_element))
                              (else
                                (Utilities|FlowControl|Delay 0.01)
                                (goto _label_4))))
                          (Variables|/Game/Chess/Blueprints/ChessPieces/BP_PieceParent.BP_PieceParent_C|SetFinalMovesAfterSimulationReady _pieceonsquare true)
                          (if (> (Utilities|Array|Length (Variables|/Game/Chess/Blueprints/ChessPieces/BP_PieceParent.BP_PieceParent_C|GetFinalAvailableMovesAfterSimulation _pieceonsquare)) 0)
                            (for _array_element_2 (Variables|/Game/Chess/Blueprints/ChessPieces/BP_PieceParent.BP_PieceParent_C|GetFinalAvailableMovesAfterSimulation _pieceonsquare)
                              (CallFunction|HighlightAvailableMoves _array_element_2)))
                          (else
                            (Utilities|FlowControl|Delay 0.01)
                            (goto _label_3)))
                        (else
                          (Utilities|FlowControl|Delay 0.01)
                          (goto _label_2)))
                      (else
                        (Utilities|FlowControl|Delay 0.01)
                        (goto _label))))
                  (:Is%20Not%20Valid
                    (Development|PrintString "BP_Square : Error : \"ChessBoard not found\"" true true "(R=1.000000,G=0.000000,B=0.133648,A=1.000000)")))
                (else
                  (Utilities|IsValid _chessboard :!label _label_5
                    (:Is%20Valid
                      (Utilities|IsValid (Variables|/Game/Chess/Blueprints/ChessBoard/BP_ChessBoard.BP_ChessBoard_C|GetSelectedSquare _chessboard)
                        (:Is%20Valid
                          (if (!= (Variables|/Game/Chess/Blueprints/ChessBoard/BP_ChessBoard.BP_ChessBoard_C|GetSelectedSquare _chessboard) self)
                            ;[1 1 1] Get the piece we try to move
                            (bind (_pieceonsquare_2 _valid_2) (CallFunction|FLGetPieceonSquare (Variables|/Game/Chess/Blueprints/ChessBoard/BP_ChessBoard.BP_ChessBoard_C|GetSelectedSquare _chessboard)))
                            (if _valid_2
                              (if (Variables|/Game/Chess/Blueprints/ChessPieces/BP_PieceParent.BP_PieceParent_C|GetFinalMovesAfterSimulationReady _pieceonsquare_2) :!label _label_6
                                (if (Utilities|Array|ContainsItem (Variables|/Game/Chess/Blueprints/ChessPieces/BP_PieceParent.BP_PieceParent_C|GetFinalAvailableMovesAfterSimulation _pieceonsquare_2) self)
                                  (bind _aspawn_player (Utilities|Casting|CastToBP_Chess_PlayerPawn (Game|Player|GetPlayerPawn 0)))
                                  ;[1 0 0.005228] Some other check to do before. Example: check if this can bring my king in check
                                  (Default|MovePiece _aspawn_player self _pieceonsquare_2))
                                (else
                                  (Utilities|FlowControl|Delay 0.01)
                                  (goto _label_6))))))))
                    (:Is%20Not%20Valid
                      (Development|PrintString "BP_Square : Error : \"ChessBoard ,ot found\"" true true "(R=1.000000,G=0.000000,B=0.133648,A=1.000000)")))))
              (else
                (goto _label_5)))))))))

(event Custom|HighlightAvailableMoves
  ;[1 1 1] Available highlight system
  (Variables|Default|SetAvailableHightLight true)
  (Rendering|Material|SetMaterial (Variables|Default|GetPlane) 0 "/Game/Chess/Materials/MI_HighLighted_Available_Inst.MI_HighLighted_Available_Inst"))

(event Custom|UnClicked
  ;[1 1 1] Highlight system
  (Variables|Default|SetClicked false)
  (Variables|Default|SetAvailableHightLight false)
  (Rendering|Material|SetMaterial (Variables|Default|GetPlane) 0 (Variables|Default|GetMaterialInit)))

(event Custom|InitMaterials
  (bind _plane (Variables|Default|GetPlane))
  (if (or (and (> (Math|Integer|%(Integer) (Variables|Default|GetX) 2) 0) (> (Math|Integer|%(Integer) (Variables|Default|GetY) 2) 0)) (and (not (> (Math|Integer|%(Integer) (Variables|Default|GetX) 2) 0)) (not (> (Math|Integer|%(Integer) (Variables|Default|GetY) 2) 0))))
    (Rendering|Material|SetMaterial _plane 0 "/Game/Chess/Materials/M_BlackCase.M_BlackCase")
    (else
      (Rendering|Material|SetMaterial _plane 0 "/Game/Chess/Materials/MI_ColorMatrerial_White_Inst.MI_ColorMatrerial_White_Inst"))))

(event EventBeginPlay
  (Utilities|FlowControl|Sequence
    (:then_0
      (Utilities|FlowControl|Delay 0.5)
      (Variables|Default|SetMaterialInit (Rendering|Material|GetMaterial (Variables|Default|GetPlane) 0))
      (Variables|Default|SetGameReady true)
      (if (Variables|Default|GetShowCaseName)
        (Rendering|Components|TextRender|SetText (Variables|Default|GetTextRender) (Utilities|Text|ToText(String) (Utilities|String|Append (Utilities|String|GetSubstring "ABCDEFGHIJKLMNOPQRSTUVWXYZ" (- (Variables|Default|GetX) 1)) (Utilities|String|ToString(Integer) (Variables|Default|GetY))))))
      ;[1 1 1] Add coordonnates in Tag => make the dev easier
      (Utilities|Array|Add (Variables|Actor|GetTags self) (Utilities|String|StringToName (Utilities|String|Append (Utilities|String|ToString(Integer) (Variables|Default|GetX)) (Utilities|String|ToString(Integer) (Variables|Default|GetY))))))
    (:then_1
      (bind _asgs_game_state (Utilities|Casting|CastToBP_Chess_GameState (Game|GetGameState) :!label _label)
        (:then
          (Variables|Default|SetAs%20GS%20Game%20State _asgs_game_state))
        (:CastFailed
          (Utilities|FlowControl|Delay 0.2)
          (goto _label))))
    (:then_2
      (CallFunction|InitMaterials)
      (Utilities|FlowControl|Delay 0.5)
      (CallFunction|InitMaterials))))

(fn ConstructionScript)

(fn DetectPieceandSquare
  (LocalVariables|SetPiece 0)
  (bind _outactors (Actor|GetAllActorsOfClass "/Game/Chess/Blueprints/ChessPieces/BP_PieceParent.BP_PieceParent_C"))
  (bind _array_element (Utilities|Array|ForEachLoopwithBreak _outactors :!label _label)
    (:LoopBody
      (if (and (== (Variables|/Game/Chess/Blueprints/ChessPieces/BP_PieceParent.BP_PieceParent_C|GetCurrentX _array_element) (Variables|Default|GetX)) (== (Variables|/Game/Chess/Blueprints/ChessPieces/BP_PieceParent.BP_PieceParent_C|GetCurrentY _array_element) (Variables|Default|GetY)))
        (LocalVariables|SetPiece _array_element)
        (goto _label Break)))
    (:Completed
      (return (LocalVariables|GetPiece)))))

(fn UnSelectOtherSquares
  ;[1 1 1] UnSelect all other squares
  (bind _outactors (Actor|GetAllActorsOfClass "BP_Square_C"))
  (for _array_element _outactors
    (if (!= _array_element self)
      (CallFunction|UnClicked _array_element)))
  (return))

(fn OnRepX)

(fn OnRepY)

(fn OnRepChessBoard)

(fn OnRepMaterialInit)
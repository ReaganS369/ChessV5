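; Base Blueprint for chess pieces, with replicated color, coordinates and move count, plus move-query events for child pieces to implement.
; Color initialization applies white or black materials and rotates the piece once on the server.
; Move simulation temporarily changes coordinates, hides captures (including en passant) via a simulated-death flag, polls the king's dangerous squares for check, then restores state.
; A filtering event removes enemy king squares from available moves.
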(event Custom|PieceColorInit
  (bind _skeletalmesh (Variables|Default|GetSkeletalMesh))
  (bind _staticmesh (Variables|Default|GetStaticMesh))
  (switch int (Variables|Default|GetPieceColor)
    (:1
      (bind _returnvalue (Rendering|Material|CreateDynamicMaterialInstance "/Game/Chess/Materials/MI_ColorMatrerial_White_Attenuation_Inst.MI_ColorMatrerial_White_Attenuation_Inst" "None" "None" :!class /Script/Engine.KismetMaterialLibrary))
      (Rendering|Material|SetMaterial _staticmesh 0 _returnvalue)
      (Rendering|Material|SetMaterial _skeletalmesh 0 _returnvalue))
    (:2
      (bind _returnvalue_2 (Rendering|Material|CreateDynamicMaterialInstance "/Game/Chess/Materials/MI_BlackPiece_Inst.MI_BlackPiece_Inst" "None" "None" :!class /Script/Engine.KismetMaterialLibrary))
      (Rendering|Material|SetMaterial _staticmesh 0 _returnvalue_2)
      (Rendering|Material|SetMaterial _skeletalmesh 0 _returnvalue_2)))
  (Utilities|FlowControl|DoOnce false
    (:Completed
      (if (Networking|IsServer)
        (switch int (Variables|Default|GetPieceColor)
          (:1
            (Class|Actor|AddActorWorldRotation (Math|Rotator|MakeRotator 0.0 0.0 -9e+01)))
          (:2
            (Class|Actor|AddActorWorldRotation (Math|Rotator|MakeRotator 0.0 0.0 9e+01))))))))

(event Custom|GetAvailableMoves
  ;[1 0 0.01933] Don't remove it
  ; It is needed in childs pieces !
)

(event Custom|GetAvailableMoveAfterKingCheck
  ;[1 1 1] Remove the opposite king in availables moves after king check array
  (Utilities|Array|Clear (Variables|Default|GetAvailableMovesAfterKingCheck))
  (Variables|Default|SetAvailableMovesAfterKingCheck (Variables|Default|GetAvailableMovesBeforeKingCheck))
  (bind _outactors (Actor|GetAllActorsOfClass "/Game/Chess/Blueprints/ChessPieces/BP_Piece_Child_king.BP_Piece_Child_king_C"))
  (for _array_element _outactors
    (if (!= (Variables|Default|GetPieceColor) (Variables|BP_PieceParent_C|GetPieceColor _array_element))
      (bind _square (CallFunction|FLGetSquareUnderPiece _array_element))
      (Utilities|Array|RemoveItem (Variables|Default|GetAvailableMovesAfterKingCheck) _square)))
  (Variables|Default|SetAivailableMovesAfterKingCheckReady true))

(event Custom|S_MovesAccountIncrementation
  (bind _result (Math|Integer|IncrementInt (Variables|Default|GetPieceMovesAccount))
    (:%20%20
      (Variables|Default|SetPieceMovesAccount _result))))

(event Custom|MovesAccountIncrementation
  (CallFunction|SMovesAccountIncrementation))

(event Custom|GetFinalAvailableMoves
  ;[1 0 0.01933] Don't remove it
  ; It is needed in childs pieces !
)

(event Custom|SimulateMove
  (params (SquareToSimulate :type BP%20Square%20Object%20Reference))
  ;[1 1 1] Now we have to call this when checking available moves
  (Utilities|IsValid SquareToSimulate
    (:Is%20Valid
      (Variables|Default|SetSquare%20to%20Simulate SquareToSimulate)
      (Variables|Default|SetMoveSimulationFinished false)
      (Variables|Default|SetSimulatedKingInDanger false)
      (Variables|Default|SetSimulatedTakenPiece 0)
      ;[1 1 1] Save the situation of the piece before the simulation
      (Variables|Default|SetxBeforeSimulation (Variables|Default|GetCurrentX))
      (Variables|Default|SetyBeforeSimulation (Variables|Default|GetCurrentY))
      ;[1 1 1] Simulate we are eating this piece (the piece will simulate it does not exist anymore on the chess board)
      (bind (_pieceonsquare _valid) (CallFunction|FLGetPieceonSquarebyCoordonnates (Variables|/Game/Chess/Blueprints/ChessBoard/BP_Square.BP_Square_C|GetX (Variables|Default|GetSquare%20to%20Simulate)) (Variables|/Game/Chess/Blueprints/ChessBoard/BP_Square.BP_Square_C|GetY (Variables|Default|GetSquare%20to%20Simulate))))
      (if _valid
        (if (!= _pieceonsquare "/Game/Chess/Blueprints/ChessPieces/BP_Piece_Child_king.BP_Piece_Child_king")
          (Variables|BP_PieceParent_C|SetSimulatedTakenPiece self _pieceonsquare)
          (Variables|BP_PieceParent_C|SetisSimulatingDeath (Variables|Default|GetSimulatedTakenPiece) true)
          ;[1 1 1] Simulate a move
          (Variables|Default|SetCurrentX (Variables|/Game/Chess/Blueprints/ChessBoard/BP_Square.BP_Square_C|GetX (Variables|Default|GetSquare%20to%20Simulate)) :!label _label)
          (Variables|Default|SetCurrentY (Variables|/Game/Chess/Blueprints/ChessBoard/BP_Square.BP_Square_C|GetY (Variables|Default|GetSquare%20to%20Simulate)))
          ;[1 1 1] Check if the king is in check during simulated move
          (bind _king (CallFunction|FLGetKing (Variables|Default|GetPieceColor)))
          (Utilities|IsValid _king
            (:Is%20Valid
              (bind _square (CallFunction|FLGetSquareUnderPiece _king))
              (Default|ComputeDangerousSquares _king)
              (if (Variables|/Game/Chess/Blueprints/ChessPieces/BP_Piece_Child_king.BP_Piece_Child_king_C|GetDangerousSquaresReady _king) :!label _label_2
                (if (Utilities|Array|ContainsItem (Variables|/Game/Chess/Blueprints/ChessPieces/BP_Piece_Child_king.BP_Piece_Child_king_C|GetDangerousSquares _king) _square)
                  (Variables|Default|SetSimulatedKingInDanger true)
                  (else
                    (Variables|Default|SetSimulatedKingInDanger false)))
                (else
                  (Utilities|FlowControl|Delay 0.01)
                  (goto _label_2))))
            (:Is%20Not%20Valid
              _))
          ;[1 1 1] Replace the pieces in the before simulation situation
          (Variables|Default|SetCurrentX (Variables|Default|GetxBeforeSimulation))
          (Variables|Default|SetCurrentY (Variables|Default|GetyBeforeSimulation))
          (Utilities|IsValid (Variables|Default|GetSimulatedTakenPiece)
            (:Is%20Valid
              (Variables|BP_PieceParent_C|SetisSimulatingDeath (Variables|Default|GetSimulatedTakenPiece) false))
            (:Is%20Not%20Valid
              _))
          (Variables|Default|SetMoveSimulationFinished true)
          (else
            (Development|PrintString "BP_Piece_Parent: \"Error : you are trying to eat a King\"" true true "(R=1.000000,G=0.000000,B=0.114252,A=1.000000)")
            (Variables|Default|SetMoveSimulationFinished true)))
        (else
          ;[1 0 0.1177 1 12] Check if EnPassant
          (if (== (Variables|Default|GetPieceType) 1)
            (switch int (Variables|Default|GetPieceColor)
              (:1
                (if (== (Variables|Default|GetCurrentY) 5)
                  ;;[1 1 1] If True : A pawn is processing a diagonal move on an empty square : it's a take "en passant"
                  (if (!= (Variables|/Game/Chess/Blueprints/ChessBoard/BP_Square.BP_Square_C|GetX (Variables|Default|GetSquare%20to%20Simulate)) (Variables|Default|GetCurrentX))
                    (bind (_pieceonsquare_2 _valid_2) (CallFunction|FLGetPieceonSquarebyCoordonnates (Variables|/Game/Chess/Blueprints/ChessBoard/BP_Square.BP_Square_C|GetX (Variables|Default|GetSquare%20to%20Simulate)) (+ (Variables|/Game/Chess/Blueprints/ChessBoard/BP_Square.BP_Square_C|GetY (Variables|Default|GetSquare%20to%20Simulate)) -1)))
                    (if _valid_2
                      (Variables|BP_PieceParent_C|SetSimulatedTakenPiece self _pieceonsquare_2)
                      (else
                        (goto _label)))
                    (else
                      (goto _label)))
                  (else
                    (goto _label))))
              (:2
                (if true
                  (if (!= (Variables|/Game/Chess/Blueprints/ChessBoard/BP_Square.BP_Square_C|GetX (Variables|Default|GetSquare%20to%20Simulate)) (Variables|Default|GetCurrentX))
                    (bind (_pieceonsquare_3 _valid_3) (CallFunction|FLGetPieceonSquarebyCoordonnates (Variables|/Game/Chess/Blueprints/ChessBoard/BP_Square.BP_Square_C|GetX (Variables|Default|GetSquare%20to%20Simulate)) (+ (Variables|/Game/Chess/Blueprints/ChessBoard/BP_Square.BP_Square_C|GetY (Variables|Default|GetSquare%20to%20Simulate)) 1)))
                    (if _valid_3
                      (Variables|BP_PieceParent_C|SetSimulatedTakenPiece self _pieceonsquare_3)
                      (else
                        (goto _label)))
                    (else
                      (goto _label)))
                  (else
                    (goto _label)))))
            (Variables|BP_PieceParent_C|SetisSimulatingDeath (Variables|Default|GetSimulatedTakenPiece) true)
            (goto _label)
            (else
              (goto _label))))))
    (:Is%20Not%20Valid
      (Development|PrintString "BP_Piece_Parent: \"Error : Square To Simulate Not Found\"" true true "(R=1.000000,G=0.000000,B=0.114252,A=1.000000)"))))

(event EventBeginPlay
  (bind _asbp_chess_game_state (Utilities|Casting|CastToBP_Chess_GameState (Game|GetGameState))
    (:then
      (Variables|Default|SetAs%20GS%20Game%20State _asbp_chess_game_state))
    (:CastFailed
      (Development|PrintString "BP_PieceParent: \"GS_GameState Not Found\"" true true "(R=1.000000,G=0.057504,B=0.000000,A=1.000000)" 2e+02))))

(fn ConstructionScript)

(fn OnRepPieceMovesAccount)

(fn OnRepCurrentY
  ;[1 1 1] Be careful before using this since it is used in the move simulation
)

(fn OnRepCurrentX
  ;[1 1 1] Be careful before using this since it is used in the move simulation
)

(fn OnRepPieceColor
  (CallFunction|PieceColorInit))

(fn OnRepTurnwhenLastMove)
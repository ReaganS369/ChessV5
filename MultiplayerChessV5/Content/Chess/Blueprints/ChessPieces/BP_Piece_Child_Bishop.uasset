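; Bishop chess piece child Blueprint that computes the squares the bishop can move to and threaten.
; GetAvailableMoves walks four diagonals from the current square within BP_ChessBoard bounds, using CheckSquare's Break/Continue exits to stop at blockers.
; CheckSquare records every reached square as hostile to the opposing king, including defended allies, but only empty or enemy squares as moves.
; GetFinalAvailableMoves passes the king-check-filtered list on as pre-simulation final moves and flags it ready.
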(event EventGetFinalAvailableMoves
  ;[1 0 0.04707] Get final moves
  (Variables|Default|SetFinalAvailableMovesBeforeSimulation (Variables|Default|GetAvailableMovesAfterKingCheck))
  (Variables|Default|SetFinalAvailableMovesReady true))

(event EventGetAvailableMoves
  ;[1 1 1] Initialization
  (Variables|Default|SetAvailableMovesBeforeKingCheckReady false)
  (Variables|Default|SetAivailableMovesAfterKingCheckReady false)
  (Variables|Default|SetFinalAvailableMovesReady false)
  (Utilities|Array|Clear (Variables|Default|GetAvailableMovesBeforeKingCheck))
  (Utilities|Array|Clear (Variables|Default|GetFinalAvailableMovesBeforeSimulation))
  ;[0 1 0.9615] This will contain the moves that could put the opposite king in danger
  (Utilities|Array|Clear (Variables|Default|GetHostilMovesForOppositKing))
  (bind _returnvalue (Actor|GetActorOfClass "/Game/Chess/Blueprints/ChessBoard/BP_ChessBoard.BP_ChessBoard_C"))
  (Utilities|IsValid _returnvalue
    (:Is%20Valid
      (Variables|Default|SetChessBoard _returnvalue)
      ;[1 1 1] FrontRight Diagonal Check
      (Variables|Default|SetxIndex (+ (Variables|Default|GetCurrentX) 1))
      (Variables|Default|SetyIndex (+ (Variables|Default|GetCurrentY) 1))
      (Variables|Default|SetBreak false)
      (while (Math|Boolean|ANDBoolean (<= (Variables|Default|GetxIndex) (Variables|/Game/Chess/Blueprints/ChessBoard/BP_ChessBoard.BP_ChessBoard_C|GetMaxX (Variables|Default|GetChessBoard))) (<= (Variables|Default|GetyIndex) (Variables|/Game/Chess/Blueprints/ChessBoard/BP_ChessBoard.BP_ChessBoard_C|GetMaxY (Variables|Default|GetChessBoard))) (not (Variables|Default|GetBreak)))
        (Utilities|CheckSquare (Variables|Default|GetxIndex) (Variables|Default|GetyIndex) (Variables|Default|GetPieceColor)
          (:Break
            (Variables|Default|SetBreak true))
          (:Continue
            (bind _result (Math|Integer|IncrementInt (Variables|Default|GetxIndex))
              (:%20%20
                (Variables|Default|SetxIndex _result)
                (bind _result_2 (Math|Integer|IncrementInt (Variables|Default|GetyIndex))
                  (:%20%20
                    (Variables|Default|SetyIndex _result_2))))))))
      ;[1 1 1] FrontLeft Diagonal Check
      (Variables|Default|SetxIndex (+ (Variables|Default|GetCurrentX) -1))
      (Variables|Default|SetyIndex (+ (Variables|Default|GetCurrentY) 1))
      (Variables|Default|SetBreak false)
      (while (Math|Boolean|ANDBoolean (>= (Variables|Default|GetxIndex) 1) (<= (Variables|Default|GetyIndex) (Variables|/Game/Chess/Blueprints/ChessBoard/BP_ChessBoard.BP_ChessBoard_C|GetMaxY (Variables|Default|GetChessBoard))) (not (Variables|Default|GetBreak)))
        (Utilities|CheckSquare (Variables|Default|GetxIndex) (Variables|Default|GetyIndex) (Variables|Default|GetPieceColor)
          (:Break
            (Variables|Default|SetBreak true))
          (:Continue
            (bind _result_3 (Math|Integer|DecrementInt (Variables|Default|GetxIndex))
              (:%20%20
                (Variables|Default|SetxIndex _result_3)
                (bind _result_4 (Math|Integer|IncrementInt (Variables|Default|GetyIndex))
                  (:%20%20
                    (Variables|Default|SetyIndex _result_4))))))))
      ;[1 1 1] BackLeft Diagonal Check
      (Variables|Default|SetxIndex (+ (Variables|Default|GetCurrentX) -1))
      (Variables|Default|SetyIndex (+ (Variables|Default|GetCurrentY) -1))
      (Variables|Default|SetBreak false)
      (while (Math|Boolean|ANDBoolean (>= (Variables|Default|GetxIndex) 1) (>= (Variables|Default|GetyIndex) 1) (not (Variables|Default|GetBreak)))
        (Utilities|CheckSquare (Variables|Default|GetxIndex) (Variables|Default|GetyIndex) (Variables|Default|GetPieceColor)
          (:Break
            (Variables|Default|SetBreak true))
          (:Continue
            (bind _result_5 (Math|Integer|DecrementInt (Variables|Default|GetxIndex))
              (:%20%20
                (Variables|Default|SetxIndex _result_5)
                (bind _result_6 (Math|Integer|DecrementInt (Variables|Default|GetyIndex))
                  (:%20%20
                    (Variables|Default|SetyIndex _result_6))))))))
      ;[1 1 1] BackRight Diagonal Check
      (Variables|Default|SetxIndex (+ (Variables|Default|GetCurrentX) 1))
      (Variables|Default|SetyIndex (+ (Variables|Default|GetCurrentY) -1))
      (Variables|Default|SetBreak false)
      (while (Math|Boolean|ANDBoolean (<= (Variables|Default|GetxIndex) (Variables|/Game/Chess/Blueprints/ChessBoard/BP_ChessBoard.BP_ChessBoard_C|GetMaxX (Variables|Default|GetChessBoard))) (>= (Variables|Default|GetyIndex) 1) (not (Variables|Default|GetBreak)))
        (Utilities|CheckSquare (Variables|Default|GetxIndex) (Variables|Default|GetyIndex) (Variables|Default|GetPieceColor)
          (:Break
            (Variables|Default|SetBreak true))
          (:Continue
            (bind _result_7 (Math|Integer|IncrementInt (Variables|Default|GetxIndex))
              (:%20%20
                (Variables|Default|SetxIndex _result_7)
                (bind _result_8 (Math|Integer|DecrementInt (Variables|Default|GetyIndex))
                  (:%20%20
                    (Variables|Default|SetyIndex _result_8))))))))
      ;[1 1 1] Build Available Move After King Check array in parent Blueprint: it removes the opposite king(s) square(s) from a second array but keep the first one named "available move before king check" so we will be able to easy check for "check" situation. I hope it is understandable :D : look in the parent class if not
      (Variables|Default|SetAvailableMovesBeforeKingCheckReady true))
    (:Is%20Not%20Valid
      (Development|PrintString "BP_PieceChild_Bishop : \"BP_ChessBoard Not Found\"" true true "(R=1.000000,G=0.000000,B=0.095397,A=1.000000)" 2e+02))))

(fn ConstructionScript
  (|CallParentFunction))
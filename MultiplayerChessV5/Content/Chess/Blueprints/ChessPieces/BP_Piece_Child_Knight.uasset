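; Knight chess piece Blueprint, a child of a base piece class, that computes the squares the knight can move to.
; GetAvailableMoves runs a CheckSquare macro on the eight L-shaped offsets, recording every existing square as hostile to the opposing king and empty or enemy-held ones as available moves.
; Ready flags mark each stage, and GetFinalAvailableMoves copies the parent's king-checked list into the pre-simulation array.
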(event EventGetFinalAvailableMoves
  ;[1 0 0.04707] Get final moves
  (Variables|Default|SetFinalAvailableMovesBeforeSimulation (Variables|Default|GetAvailableMovesAfterKingCheck))
  (Variables|Default|SetFinalAvailableMovesReady true))

(event EventGetAvailableMoves
  ;[1 1 1] Initialization
  (Variables|Default|SetAvailableMovesBeforeKingCheckReady false)
  (Variables|Default|SetAivailableMovesAfterKingCheckReady false)
  (Variables|Default|SetFinalAvailableMovesReady false)
  (Utilities|Array|Clear (Variables|Default|GetAvailableMovesBeforeKingCheck))
  (Utilities|Array|Clear (Variables|Default|GetFinalAvailableMovesBeforeSimulation))
  ;[0 1 0.9615] This will contain the moves that could put the opposite king in danger
  (Utilities|Array|Clear (Variables|Default|GetHostilMovesForOppositKing))
  (bind _returnvalue (Actor|GetActorOfClass "/Game/Chess/Blueprints/ChessBoard/BP_ChessBoard.BP_ChessBoard_C"))
  (Utilities|IsValid _returnvalue
    (:Is%20Valid
      (Variables|Default|SetChessBoard _returnvalue)
      (Utilities|CheckSquare (+ (Variables|Default|GetCurrentX) 1) (+ (Variables|Default|GetCurrentY) 2) (Variables|Default|GetPieceColor)
        (:Break
          _)
        (:Continue
          _))
      (Utilities|CheckSquare (+ (Variables|Default|GetCurrentX) -1) (+ (Variables|Default|GetCurrentY) 2) (Variables|Default|GetPieceColor)
        (:Break
          _)
        (:Continue
          _))
      (Utilities|CheckSquare (+ (Variables|Default|GetCurrentX) 1) (+ (Variables|Default|GetCurrentY) -2) (Variables|Default|GetPieceColor)
        (:Break
          _)
        (:Continue
          _))
      (Utilities|CheckSquare (+ (Variables|Default|GetCurrentX) -1) (+ (Variables|Default|GetCurrentY) -2) (Variables|Default|GetPieceColor)
        (:Break
          _)
        (:Continue
          _))
      (Utilities|CheckSquare (+ (Variables|Default|GetCurrentX) 2) (+ (Variables|Default|GetCurrentY) 1) (Variables|Default|GetPieceColor)
        (:Break
          _)
        (:Continue
          _))
      (Utilities|CheckSquare (+ (Variables|Default|GetCurrentX) -2) (+ (Variables|Default|GetCurrentY) 1) (Variables|Default|GetPieceColor)
        (:Break
          _)
        (:Continue
          _))
      (Utilities|CheckSquare (+ (Variables|Default|GetCurrentX) 2) (+ (Variables|Default|GetCurrentY) -1) (Variables|Default|GetPieceColor)
        (:Break
          _)
        (:Continue
          _))
      (Utilities|CheckSquare (+ (Variables|Default|GetCurrentX) -2) (+ (Variables|Default|GetCurrentY) -1) (Variables|Default|GetPieceColor)
        (:Break
          _)
        (:Continue
          _))
      ;[1 1 1] Build Available Move After King Check array in parent Blueprint: it removes the opposite king(s) square(s) from a second array but keep the first one named "available move before king check" so we will be able to easy check for "check" situation. I hope it is understandable :D : look in the parent class if not
      (Variables|Default|SetAvailableMovesBeforeKingCheckReady true))
    (:Is%20Not%20Valid
      (Development|PrintString "BP_PieceChild_Knight : \"BP_ChessBoard Not Found\""))))

(fn ConstructionScript
  (|CallParentFunction))
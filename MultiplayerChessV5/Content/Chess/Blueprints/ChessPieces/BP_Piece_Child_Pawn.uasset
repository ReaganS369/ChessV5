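; Pawn chess piece Blueprint that generates its candidate moves for the parent piece class's king-check filtering.
; GetAvailableMoves adds forward steps by color, allowing double steps from the starting rank in classic mode, anywhere otherwise.
; ContinueGettingAvailableMoves adds diagonal captures and optional en passant, while PawnCheckSquare records all diagonals as hostile to the opposing king.
; Ready flags mark each stage, with GetFinalAvailableMoves copying the king-checked list for later simulation.
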(event Custom|ContinueGettingAvailableMoves
  ;[1 1 1] Diagonal eating - move only if it can eat opposite piece
  (switch int (Variables|Default|GetPieceColor)
    (:1
      (if (< (Variables|Default|GetCurrentY) (Variables|/Game/Chess/Blueprints/ChessBoard/BP_ChessBoard.BP_ChessBoard_C|GetMaxY (Variables|Default|GetChessBoard)))
        (Utilities|PawnCheckSquare (+ (Variables|Default|GetCurrentX) 1) (+ (Variables|Default|GetCurrentY) 1) (Variables|Default|GetPieceColor)
          (:Break
            _)
          (:Continue
            _))
        (Utilities|PawnCheckSquare (+ (Variables|Default|GetCurrentX) -1) (+ (Variables|Default|GetCurrentY) 1) (Variables|Default|GetPieceColor)
          (:Break
            _)
          (:Continue
            _))
        ;;[1 1 1] To Take "En Passant"
        (if (Variables|Default|GetToTakeEnPassantFeature)
          (if (== (Variables|Default|GetCurrentY) 5)
            (bind (_square _exists) (CallFunction|FLGetSquarebyCoordonnate (+ (Variables|Default|GetCurrentX) 1) (Variables|Default|GetCurrentY)))
            (if _exists
              (bind (_pieceonsquare _valid) (CallFunction|FLGetPieceonSquare _square))
              (if _valid
                (if (== (Variables|/Game/Chess/Blueprints/ChessPieces/BP_PieceParent.BP_PieceParent_C|GetPieceType _pieceonsquare) 1)
                  (if (== (Variables|/Game/Chess/Blueprints/BP_Chess_GameState.BP_Chess_GameState_C|GetTurnAccount (Variables|Default|GetAs%20GS%20Game%20State)) (Variables|/Game/Chess/Blueprints/ChessPieces/BP_PieceParent.BP_PieceParent_C|GetTurnWhenLastMove _pieceonsquare))
                    (bind (_square_2 _exists_2) (CallFunction|FLGetSquarebyCoordonnate (+ (Variables|Default|GetCurrentX) 1) (+ (Variables|Default|GetCurrentY) 1)))
                    (if _exists_2
                      (Utilities|Array|Add (Variables|Default|GetAvailableMovesBeforeKingCheck) _square_2))))))
            (bind (_square_3 _exists_3) (CallFunction|FLGetSquarebyCoordonnate (+ (Variables|Default|GetCurrentX) -1) (Variables|Default|GetCurrentY)))
            (if _exists_3
              (bind (_pieceonsquare_2 _valid_2) (CallFunction|FLGetPieceonSquare _square_3))
              (if _valid_2
                (if (== (Variables|/Game/Chess/Blueprints/ChessPieces/BP_PieceParent.BP_PieceParent_C|GetPieceType _pieceonsquare_2) 1)
                  (if (== (Variables|/Game/Chess/Blueprints/BP_Chess_GameState.BP_Chess_GameState_C|GetTurnAccount (Variables|Default|GetAs%20GS%20Game%20State)) (Variables|/Game/Chess/Blueprints/ChessPieces/BP_PieceParent.BP_PieceParent_C|GetTurnWhenLastMove _pieceonsquare_2))
                    (bind (_square_4 _exists_4) (CallFunction|FLGetSquarebyCoordonnate (+ (Variables|Default|GetCurrentX) -1) (+ (Variables|Default|GetCurrentY) 1)))
                    (if _exists_4
                      (Utilities|Array|Add (Variables|Default|GetAvailableMovesBeforeKingCheck) _square_4))))))
            (CallFunction|FinishGettingAvailableMoves)
            (else
              (CallFunction|FinishGettingAvailableMoves :!label _label)))
          (else
            (goto _label)))
        (else
          (CallFunction|FinishGettingAvailableMoves))))
    (:2
      (if (> (Variables|Default|GetCurrentY) 1)
        (Utilities|PawnCheckSquare (+ (Variables|Default|GetCurrentX) 1) (+ (Variables|Default|GetCurrentY) -1) (Variables|Default|GetPieceColor)
          (:Break
            _)
          (:Continue
            _))
        (Utilities|PawnCheckSquare (+ (Variables|Default|GetCurrentX) -1) (+ (Variables|Default|GetCurrentY) -1) (Variables|Default|GetPieceColor)
          (:Break
            _)
          (:Continue
            _))
        ;;[1 1 1] To Take "En Passant"
        (if (Variables|Default|GetToTakeEnPassantFeature)
          (if (== (Variables|Default|GetCurrentY) 4)
            (bind (_square_5 _exists_5) (CallFunction|FLGetSquarebyCoordonnate (+ (Variables|Default|GetCurrentX) 1) (Variables|Default|GetCurrentY)))
            (if _exists_5
              (bind (_pieceonsquare_3 _valid_3) (CallFunction|FLGetPieceonSquare _square_5))
              (if _valid_3
                (if (== (Variables|/Game/Chess/Blueprints/ChessPieces/BP_PieceParent.BP_PieceParent_C|GetPieceType _pieceonsquare_3) 1)
                  (if (== (Variables|/Game/Chess/Blueprints/BP_Chess_GameState.BP_Chess_GameState_C|GetTurnAccount (Variables|Default|GetAs%20GS%20Game%20State)) (Variables|/Game/Chess/Blueprints/ChessPieces/BP_PieceParent.BP_PieceParent_C|GetTurnWhenLastMove _pieceonsquare_3))
                    (bind (_square_6 _exists_6) (CallFunction|FLGetSquarebyCoordonnate (+ (Variables|Default|GetCurrentX) 1) (+ (Variables|Default|GetCurrentY) -1)))
                    (if _exists_6
                      (Utilities|Array|Add (Variables|Default|GetAvailableMovesBeforeKingCheck) _square_6))))))
            (bind (_square_7 _exists_7) (CallFunction|FLGetSquarebyCoordonnate (+ (Variables|Default|GetCurrentX) -1) (Variables|Default|GetCurrentY)))
            (if _exists_7
              (bind (_pieceonsquare_4 _valid_4) (CallFunction|FLGetPieceonSquare _square_7))
              (if _valid_4
                (if (== (Variables|/Game/Chess/Blueprints/ChessPieces/BP_PieceParent.BP_PieceParent_C|GetPieceType _pieceonsquare_4) 1)
                  (if (== (Variables|/Game/Chess/Blueprints/BP_Chess_GameState.BP_Chess_GameState_C|GetTurnAccount (Variables|Default|GetAs%20GS%20Game%20State)) (Variables|/Game/Chess/Blueprints/ChessPieces/BP_PieceParent.BP_PieceParent_C|GetTurnWhenLastMove _pieceonsquare_4))
                    (bind (_square_8 _exists_8) (CallFunction|FLGetSquarebyCoordonnate (+ (Variables|Default|GetCurrentX) -1) (+ (Variables|Default|GetCurrentY) -1)))
                    (if _exists_8
                      (Utilities|Array|Add (Variables|Default|GetAvailableMovesBeforeKingCheck) _square_8))))))
            (CallFunction|FinishGettingAvailableMoves)
            (else
              (CallFunction|FinishGettingAvailableMoves :!label _label_2)))
          (else
            (goto _label_2)))
        (else
          (CallFunction|FinishGettingAvailableMoves))))))

(event Custom|FinishGettingAvailableMoves
  ;[1 1 1] Build Available Move After King Check array in parent Blueprint: it removes the opposite king(s) square(s) from a second array but keep the first one named "available move before king check" so we will be able to easy check for "check" situation. I hope it is understandable :D : look in the parent class if not
  (Variables|Default|SetAvailableMovesBeforeKingCheckReady true))

(event EventGetAvailableMoves
  (bind _currenty (Variables|Default|GetCurrentY))
  (bind _currenty_2 (Variables|Default|GetCurrentY))
  ;[1 1 1] Initialization
  (Variables|Default|SetAvailableMovesBeforeKingCheckReady false)
  (Variables|Default|SetAivailableMovesAfterKingCheckReady false)
  (Variables|Default|SetFinalAvailableMovesReady false)
  (Utilities|Array|Clear (Variables|Default|GetAvailableMovesBeforeKingCheck))
  (Utilities|Array|Clear (Variables|Default|GetFinalAvailableMovesBeforeSimulation))
  ;[0 1 0.9615] This will contain the moves that could put the opposite king in danger
  (Utilities|Array|Clear (Variables|Default|GetHostilMovesForOppositKing))
  (bind _returnvalue (Actor|GetActorOfClass "/Game/Chess/Blueprints/ChessBoard/BP_ChessBoard.BP_ChessBoard_C"))
  (Utilities|IsValid _returnvalue
    (:Is%20Valid
      (Variables|Default|SetChessBoard _returnvalue)
      (switch int (Variables|Default|GetPieceColor)
        (:1
          (if (< (Variables|Default|GetCurrentY) (Variables|/Game/Chess/Blueprints/ChessBoard/BP_ChessBoard.BP_ChessBoard_C|GetMaxY (Variables|Default|GetChessBoard)))
            ;[1 1 1] Pawn Can't eat front
            (bind (_square _exists) (CallFunction|FLGetSquarebyCoordonnate (Variables|Default|GetCurrentX) (+ _currenty 1)))
            (if _exists
              (bind _valid (CallFunction|FLGetPieceonSquare _square))
              (if _valid
                (CallFunction|ContinueGettingAvailableMoves)
                (else
                  (Utilities|Array|Add (Variables|Default|GetAvailableMovesBeforeKingCheck) _square)
                  ;[1 1 1] Pawn can go 2 square front if starting from origin location and classical chess mode
                  (bind _twosquarespossible (CallFunction|TwoSquaresAuthorized))
                  (if _twosquarespossible
                    (bind (_square_2 _exists_2) (CallFunction|FLGetSquarebyCoordonnate (Variables|Default|GetCurrentX) (+ _currenty_2 2)))
                    (if _exists_2
                      (bind _valid_2 (CallFunction|FLGetPieceonSquare _square_2))
                      (if _valid_2
                        _
                        (else
                          (Utilities|Array|Add (Variables|Default|GetAvailableMovesBeforeKingCheck) _square_2)))
                      (CallFunction|ContinueGettingAvailableMoves)
                      (else
                        (CallFunction|ContinueGettingAvailableMoves :!label _label)))
                    (else
                      (CallFunction|ContinueGettingAvailableMoves :!label _label_2)))))
              (else
                (CallFunction|ContinueGettingAvailableMoves :!label _label_3)))
            (else
              (CallFunction|ContinueGettingAvailableMoves :!label _label_4))))
        (:2
          (if (> (Variables|Default|GetCurrentY) 1)
            (bind (_square_3 _exists_3) (CallFunction|FLGetSquarebyCoordonnate (Variables|Default|GetCurrentX) (- _currenty 1)))
            (if _exists_3
              (bind _valid_3 (CallFunction|FLGetPieceonSquare _square_3))
              (if _valid_3
                (CallFunction|ContinueGettingAvailableMoves)
                (else
                  (Utilities|Array|Add (Variables|Default|GetAvailableMovesBeforeKingCheck) _square_3)
                  (bind _twosquarespossible_2 (CallFunction|TwoSquaresAuthorized))
                  (if _twosquarespossible_2
                    (bind (_square_4 _exists_4) (CallFunction|FLGetSquarebyCoordonnate (Variables|Default|GetCurrentX) (- _currenty_2 2)))
                    (if _exists_4
                      (bind _valid_4 (CallFunction|FLGetPieceonSquare _square_4))
                      (if _valid_4
                        _
                        (else
                          (Utilities|Array|Add (Variables|Default|GetAvailableMovesBeforeKingCheck) _square_4)))
                      (CallFunction|ContinueGettingAvailableMoves)
                      (else
                        (goto _label)))
                    (else
                      (goto _label_2)))))
              (else
                (goto _label_3)))
            (else
              (goto _label_4))))))
    (:Is%20Not%20Valid
      (Development|PrintString "BP_PieceChild_Pawn: \"BP_ChessBoard Not Found\"" true true "(R=1.000000,G=0.057504,B=0.000000,A=1.000000)" 2e+02))))

(event EventGetFinalAvailableMoves
  ;[1 0 0.04707] Get final moves
  (Variables|Default|SetFinalAvailableMovesBeforeSimulation (Variables|Default|GetAvailableMovesAfterKingCheck))
  (Variables|Default|SetFinalAvailableMovesReady true))

(fn ConstructionScript
  (|CallParentFunction))

(fn TwoSquaresAuthorized
  (bind _asbp_chess_game_state (Utilities|Casting|CastToBP_Chess_GameState (Game|GetGameState))
    (:then
      (if (Variables|/Game/Chess/Blueprints/BP_Chess_GameState.BP_Chess_GameState_C|GetClassicChess _asbp_chess_game_state)
        (return (or (and (== (Variables|Default|GetPieceColor) 1) (== (Variables|Default|GetCurrentY) 2)) (and (== (Variables|Default|GetPieceColor) 2) (== (Variables|Default|GetCurrentY) 7))))
        (else
          (return true))))
    (:CastFailed
      (Development|PrintString (Utilities|String|Append (Utilities|GetDisplayName self) " TwoSquaresAuthorizedFunction " "GS_GameState not found") true true "(R=0.000000,G=0.660000,B=1.000000,A=1.000000)" 5.0))))
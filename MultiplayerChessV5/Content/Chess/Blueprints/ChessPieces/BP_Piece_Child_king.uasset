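; King chess piece that computes its legal moves, including castling, before a later simulation step.
; A CheckSquare macro gathers the eight adjacent squares as candidate moves and as threats to the opposing king.
; The final pass removes squares threatened by opposing pieces, polling ready flags with short Delays.
; It then adds castling moves when king and rook are unmoved, the path is clear and safe, and FEN flags allow it.
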(event Custom|ComputeDangerousSquares
  (Variables|Default|SetDangerousSquaresReady false)
  (Utilities|Array|Clear (Variables|Default|GetDangerousSquares))
  (bind _computedpieces (CallFunction|FLComputeAllOppositeAvailableMoveBeforeKingCheck (Variables|Default|GetPieceColor)))
  (if (> (Utilities|Array|Length _computedpieces) 0)
    (for _array_element _computedpieces
      (if (Variables|/Game/Chess/Blueprints/ChessPieces/BP_PieceParent.BP_PieceParent_C|GetAvailableMovesBeforeKingCheckReady _array_element) :!label _label
        (if (not (Variables|/Game/Chess/Blueprints/ChessPieces/BP_PieceParent.BP_PieceParent_C|GetisSimulatingDeath _array_element))
          (Utilities|Array|AppendArray (Variables|Default|GetDangerousSquares) (Variables|/Game/Chess/Blueprints/ChessPieces/BP_PieceParent.BP_PieceParent_C|GetHostilMovesForOppositKing _array_element)))
        (else
          (Utilities|FlowControl|Delay 0.01)
          (goto _label)))))
  (Variables|Default|SetDangerousSquaresReady true))

(event EventBeginPlay
  (|CallParentFunction) ; This node is disabled and will not be called.\nDrag off pins to build functionality.
)

(event EventGetFinalAvailableMoves
  (bind _rooksreadyforcasteling (Variables|Default|GetRooksReadyForCasteling))
  (Utilities|Array|Clear (Variables|Default|GetFinalAvailableMovesBeforeSimulation))
  (bind _output_get (Variables|Default|SetFinalAvailableMovesBeforeSimulation (Variables|Default|GetAvailableMovesAfterKingCheck)))
  (if (> (Utilities|Array|Length _output_get) 0)
    (CallFunction|ComputeDangerousSquares)
    (if (Variables|Default|GetDangerousSquaresReady) :!label _label
      ;[1 1 1] Delete All Dangerous Squares from King Availables moves
      (for _array_element (Variables|Default|GetDangerousSquares)
        (Utilities|Array|RemoveItem (Variables|Default|GetFinalAvailableMovesBeforeSimulation) _array_element))
      (else
        (Utilities|FlowControl|Delay 0.01)
        (goto _label))))
  ;[0 0.9023 1] Casteling Check
  (if (not (and (Variables|Default|GetSmallCastlePreventedByFEN) (Variables|Default|GetLargeCastlePreventedByFEN)))
    ;;[1 1 1 1 12] True: King Ready for casteling
    (if (== (Variables|Default|GetTurnWhenLastMove) 0)
      (switch int (Variables|Default|GetPieceColor)
        (:1
          (if (and (== (Variables|Default|GetCurrentX) 5) (== (Variables|Default|GetCurrentY) 1))
            (Utilities|Array|Clear (Variables|Default|GetRooksReadyForCasteling) :!label _label_2)
            (bind _outactors (Actor|GetAllActorsOfClass "/Game/Chess/Blueprints/ChessPieces/BP_Piece_Child_Rook.BP_Piece_Child_Rook_C"))
            (for _array_element_2 _outactors
              (if (and (== (Variables|/Game/Chess/Blueprints/ChessPieces/BP_PieceParent.BP_PieceParent_C|GetPieceColor _array_element_2) (Variables|Default|GetPieceColor)) (== (Variables|/Game/Chess/Blueprints/ChessPieces/BP_PieceParent.BP_PieceParent_C|GetTurnWhenLastMove _array_element_2) 0))
                (switch int (Variables|/Game/Chess/Blueprints/ChessPieces/BP_PieceParent.BP_PieceParent_C|GetPieceColor _array_element_2)
                  (:1
                    (if (== (Variables|/Game/Chess/Blueprints/ChessPieces/BP_PieceParent.BP_PieceParent_C|GetCurrentY _array_element_2) 1)
                      ;;[1 1 1] True : This Rook is Ready For Casteling
                      (if (or (== (Variables|/Game/Chess/Blueprints/ChessPieces/BP_PieceParent.BP_PieceParent_C|GetCurrentX _array_element_2) 1) (== (Variables|/Game/Chess/Blueprints/ChessPieces/BP_PieceParent.BP_PieceParent_C|GetCurrentX _array_element_2) 8)) :!label _label_3
                        (Utilities|Array|Add (Variables|Default|GetRooksReadyForCasteling) _array_element_2))))
                  (:2
                    (if (== (Variables|/Game/Chess/Blueprints/ChessPieces/BP_PieceParent.BP_PieceParent_C|GetCurrentY _array_element_2) 8)
                      (goto _label_3))))))
            (if (> (Utilities|Array|Length _rooksreadyforcasteling) 0)
              (for _array_element_3 _rooksreadyforcasteling
                ;;[1 1 1] If False X = 8
                ;; True: large casteling
                ;; False: small casteling
                (if (== (Variables|/Game/Chess/Blueprints/ChessPieces/BP_PieceParent.BP_PieceParent_C|GetCurrentX _array_element_3) 1)
                  (Variables|Default|SetCastelingIncrementation -1)
                  (Variables|Default|SetMaxCastelingIndex 3)
                  (if (not (Variables|Default|GetLargeCastlePreventedByFEN))
                    (Variables|Default|SetCastelingIndex 0 :!label _label_4)
                    (Variables|Default|SetRockOk true)
                    (Utilities|FlowControl|ForLoopwithBreak 0 (Variables|Default|GetMaxCastelingIndex) :!label _label_5
                      (:LoopBody
                        (bind (_square _exists) (CallFunction|FLGetSquarebyCoordonnate (+ (Variables|Default|GetCurrentX) (* (Variables|Default|GetCastelingIncrementation) (Variables|Default|GetCastelingIndex))) (Variables|Default|GetCurrentY)))
                        (if _exists
                          (bind (_pieceonsquare _valid) (CallFunction|FLGetPieceonSquare _square))
                          (if _valid
                            (if (== self _pieceonsquare)
                              (if (< (Variables|Default|GetCastelingIndex) 3) :!label _label_6
                                (if (Utilities|Array|ContainsItem (Variables|Default|GetDangerousSquares) _square)
                                  (Variables|Default|SetRockOk false :!label _label_7)
                                  (goto _label_5 Break)
                                  (else
                                    _)))
                              (else
                                (goto _label_7)))
                            (else
                              (goto _label_6)))
                          (Variables|Default|SetCastelingIndex (+ (Variables|Default|GetCastelingIndex) 1))
                          (else
                            (goto _label_7))))
                      (:Completed
                        ;;[1 1 1] All the conditions are respected for casteling with this Rook: so we add only one move beacause the first side move has already been added by other algo
                        (if (Variables|Default|GetRockOk)
                          (bind _square_2 (CallFunction|FLGetSquarebyCoordonnate (+ (Variables|Default|GetCurrentX) (* (Variables|Default|GetCastelingIncrementation) 2)) (Variables|Default|GetCurrentY)))
                          (Utilities|Array|Add (Variables|Default|GetFinalAvailableMovesBeforeSimulation) _square_2)))))
                  (else
                    (Variables|Default|SetCastelingIncrementation 1)
                    (Variables|Default|SetMaxCastelingIndex 2)
                    (if (not (Variables|Default|GetSmallCastlePreventedByFEN))
                      (goto _label_4))))))))
        (:2
          (if (and (== (Variables|Default|GetCurrentX) 5) (== (Variables|Default|GetCurrentY) 8))
            (goto _label_2)
            (else
              _))))))
  (Variables|Default|SetFinalAvailableMovesReady true))

(event EventGetAvailableMoves
  ;[1 1 1] Initialization
  (Variables|Default|SetAvailableMovesBeforeKingCheckReady false)
  (Variables|Default|SetAivailableMovesAfterKingCheckReady false)
  (Variables|Default|SetFinalAvailableMovesReady false)
  (Utilities|Array|Clear (Variables|Default|GetAvailableMovesBeforeKingCheck))
  (Utilities|Array|Clear (Variables|Default|GetFinalAvailableMovesBeforeSimulation))
  ;[0 1 0.9615] This will contain the moves that could put the opposite king in danger
  (Utilities|Array|Clear (Variables|Default|GetHostilMovesForOppositKing))
  (bind _returnvalue (Actor|GetActorOfClass "/Game/Chess/Blueprints/ChessBoard/BP_ChessBoard.BP_ChessBoard_C"))
  (Utilities|IsValid _returnvalue
    (:Is%20Valid
      (Variables|Default|SetChessBoard _returnvalue)
      (Utilities|CheckSquare (+ (Variables|Default|GetCurrentX) 1) (Variables|Default|GetCurrentY) (Variables|Default|GetPieceColor)
        (:Break
          _)
        (:Continue
          _))
      (Utilities|CheckSquare (+ (Variables|Default|GetCurrentX) -1) (Variables|Default|GetCurrentY) (Variables|Default|GetPieceColor)
        (:Break
          _)
        (:Continue
          _))
      (Utilities|CheckSquare (Variables|Default|GetCurrentX) (+ (Variables|Default|GetCurrentY) 1) (Variables|Default|GetPieceColor)
        (:Break
          _)
        (:Continue
          _))
      (Utilities|CheckSquare (Variables|Default|GetCurrentX) (+ (Variables|Default|GetCurrentY) -1) (Variables|Default|GetPieceColor)
        (:Break
          _)
        (:Continue
          _))
      (Utilities|CheckSquare (+ (Variables|Default|GetCurrentX) 1) (+ (Variables|Default|GetCurrentY) 1) (Variables|Default|GetPieceColor)
        (:Break
          _)
        (:Continue
          _))
      (Utilities|CheckSquare (+ (Variables|Default|GetCurrentX) 1) (+ (Variables|Default|GetCurrentY) -1) (Variables|Default|GetPieceColor)
        (:Break
          _)
        (:Continue
          _))
      (Utilities|CheckSquare (+ (Variables|Default|GetCurrentX) -1) (+ (Variables|Default|GetCurrentY) 1) (Variables|Default|GetPieceColor)
        (:Break
          _)
        (:Continue
          _))
      (Utilities|CheckSquare (+ (Variables|Default|GetCurrentX) -1) (+ (Variables|Default|GetCurrentY) -1) (Variables|Default|GetPieceColor)
        (:Break
          _)
        (:Continue
          _))
      ;[1 1 1] Build Available Move After King Check array in parent Blueprint: it removes the opposite king(s) square(s) from a second array but keep the first one named "available move before king check" so we will be able to easy check for "check" situation. I hope it is understandable :D : look in the parent class if not
      (Variables|Default|SetAvailableMovesBeforeKingCheckReady true))
    (:Is%20Not%20Valid
      (Development|PrintString "BP_PieceChild_King : \"BP_ChessBoard Not Found\"" true true "(R=1.000000,G=0.006108,B=0.000000,A=1.000000)" 2e+02))))

(fn ConstructionScript
  (|CallParentFunction))

(fn OnRepSmallCastlePreventedbyFEN)

(fn OnRepLargeCastlePreventedbyFEN)
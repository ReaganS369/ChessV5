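; Blueprint function library of shared chess board queries: pieces, squares, kings and the local player's color.
; Squares are found by an actor tag built from concatenated X and Y, while pieces are found by scanning all piece actors for matching coordinates.
; Square status treats pieces simulating death as absent, and the opponent move computation skips them, supporting king-check simulation.
; A deprecated dangerous-squares query remains alongside that computation, whose results need a readiness check.
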(fn FLGetPieceonSquarebyCoordonnates
  (params (X :type Integer) (Y :type Integer))
  (LocalVariables|SetPiece 0)
  (bind _outactors (Actor|GetAllActorsOfClass 0 "/Game/Chess/Blueprints/ChessPieces/BP_PieceParent.BP_PieceParent_C"))
  (bind _array_element (Utilities|Array|ForEachLoopwithBreak _outactors :!label _label)
    (:LoopBody
      (if (and (== (Variables|/Game/Chess/Blueprints/ChessPieces/BP_PieceParent.BP_PieceParent_C|GetCurrentX _array_element) X) (== (Variables|/Game/Chess/Blueprints/ChessPieces/BP_PieceParent.BP_PieceParent_C|GetCurrentY _array_element) Y))
        (LocalVariables|SetPiece _array_element)
        (goto _label Break)))
    (:Completed
      (return (LocalVariables|GetPiece) (Utilities|IsValid (LocalVariables|GetPiece))))))

(fn FLGetPlayerColor
  (bind _asbp_chess_player_pawn (Utilities|Casting|CastToBP_Chess_PlayerPawn (Pawn|GetControlledPawn (Game|GetPlayerController 0))))
  (return (Variables|/Game/Chess/Blueprints/BP_Chess_PlayerPawn.BP_Chess_PlayerPawn_C|GetPlayerColor _asbp_chess_player_pawn)))

(fn FLGetSquarebyCoordonnate
  (params (X :type Integer) (Y :type Integer))
  (bind _outactors (Actor|GetAllActorsOfClasswithTag 0 "/Game/Chess/Blueprints/ChessBoard/BP_Square.BP_Square_C" (Utilities|String|StringToName (Utilities|String|Append (Utilities|String|ToString(Integer) X) (Utilities|String|ToString(Integer) Y)))))
  (Utilities|IsValid (Utilities|Array|Get(acopy) _outactors)
    (:Is%20Valid
      (return (Utilities|Array|Get(acopy) _outactors) true))
    (:Is%20Not%20Valid
      (return 0 false))))

(fn FLGetPieceonSquare
  (params (Bp_Square :type BP%20Square%20Object%20Reference))
  (Utilities|IsValid Bp_Square
    (:Is%20Valid
      (LocalVariables|SetPiece 0)
      (bind _outactors (Actor|GetAllActorsOfClass 0 "/Game/Chess/Blueprints/ChessPieces/BP_PieceParent.BP_PieceParent_C"))
      (bind _array_element (Utilities|Array|ForEachLoopwithBreak _outactors :!label _label)
        (:LoopBody
          (if (and (== (Variables|/Game/Chess/Blueprints/ChessPieces/BP_PieceParent.BP_PieceParent_C|GetCurrentX _array_element) (Variables|/Game/Chess/Blueprints/ChessBoard/BP_Square.BP_Square_C|GetX Bp_Square)) (== (Variables|/Game/Chess/Blueprints/ChessPieces/BP_PieceParent.BP_PieceParent_C|GetCurrentY _array_element) (Variables|/Game/Chess/Blueprints/ChessBoard/BP_Square.BP_Square_C|GetY Bp_Square)))
            (LocalVariables|SetPiece _array_element)
            (goto _label Break)))
        (:Completed
          (return (LocalVariables|GetPiece) (Utilities|IsValid (LocalVariables|GetPiece))))))))

(fn FLCheckSquareStatus
  (params (X :type Integer) (Y :type Integer) (MyPieceColor :type Integer))
  (bind _outactors (Actor|GetAllActorsOfClasswithTag 0 "/Game/Chess/Blueprints/ChessBoard/BP_Square.BP_Square_C" (Utilities|String|StringToName (Utilities|String|Append (Utilities|String|ToString(Integer) X) (Utilities|String|ToString(Integer) Y)))))
  (Utilities|IsValid (Utilities|Array|Get(acopy) _outactors)
    (:Is%20Valid
      (bind (_pieceonsquare _valid) (CallFunction|FLGetPieceonSquare (Utilities|Array|Get(acopy) _outactors)))
      (if _valid
        (if (Variables|/Game/Chess/Blueprints/ChessPieces/BP_PieceParent.BP_PieceParent_C|GetisSimulatingDeath _pieceonsquare)
          (return true false false (Utilities|Array|Get(acopy) _outactors))
          (else
            (return true true (== (Variables|/Game/Chess/Blueprints/ChessPieces/BP_PieceParent.BP_PieceParent_C|GetPieceColor _pieceonsquare) MyPieceColor) (Utilities|Array|Get(acopy) _outactors))))
        (else
          (return true false false (Utilities|Array|Get(acopy) _outactors)))))
    (:Is%20Not%20Valid
      (return false false false 0))))

(fn FLGetSquareUnderPiece
  (params (Piece :type BP%20Piece%20Parent%20Object%20Reference))
  (bind _outactors (Actor|GetAllActorsOfClasswithTag 0 "/Game/Chess/Blueprints/ChessBoard/BP_Square.BP_Square_C" (Utilities|String|StringToName (Utilities|String|Append (Utilities|String|ToString(Integer) (Variables|/Game/Chess/Blueprints/ChessPieces/BP_PieceParent.BP_PieceParent_C|GetCurrentX Piece)) (Utilities|String|ToString(Integer) (Variables|/Game/Chess/Blueprints/ChessPieces/BP_PieceParent.BP_PieceParent_C|GetCurrentY Piece))))))
  (if (> (Utilities|Array|Length _outactors) 0)
    (return (Utilities|Array|Get(acopy) _outactors))))

(fn DEPRECATEDFLGetAllDangerousSquareforMyKing
  (params (Color :type Integer))
  (Utilities|Array|Clear (LocalVariables|GetDangerousSquares))
  (bind _outactors (Actor|GetAllActorsOfClass 0 "/Game/Chess/Blueprints/ChessPieces/BP_PieceParent.BP_PieceParent_C"))
  (for _array_element _outactors
    (if (!= (Variables|/Game/Chess/Blueprints/ChessPieces/BP_PieceParent.BP_PieceParent_C|GetPieceColor _array_element) Color)
      (Default|GetAvailableMoves _array_element)))
  (for _array_element_2 _outactors
    (Utilities|Array|AppendArray (LocalVariables|GetDangerousSquares) (Variables|/Game/Chess/Blueprints/ChessPieces/BP_PieceParent.BP_PieceParent_C|GetAvailableMovesBeforeKingCheck _array_element_2)))
  (return (LocalVariables|GetDangerousSquares)))

(fn FLComputeAllOppositeAvailableMoveBeforeKingCheck
  (params (Color :type Integer))
  (Utilities|Array|Clear (LocalVariables|GetComputed))
  (bind _outactors (Actor|GetAllActorsOfClass 0 "/Game/Chess/Blueprints/ChessPieces/BP_PieceParent.BP_PieceParent_C"))
  (for _array_element _outactors
    (if (!= (Variables|/Game/Chess/Blueprints/ChessPieces/BP_PieceParent.BP_PieceParent_C|GetPieceColor _array_element) Color)
      (if (not (Variables|/Game/Chess/Blueprints/ChessPieces/BP_PieceParent.BP_PieceParent_C|GetisSimulatingDeath _array_element))
        (Default|GetAvailableMoves _array_element)
        (Utilities|Array|Add (LocalVariables|GetComputed) _array_element))))
  ;[1 1 1 1 15] Need to check if ready before using results
  (return (LocalVariables|GetComputed)))

(fn FLGetKing
  (params (Color :type Integer))
  (bind _outactors (Actor|GetAllActorsOfClass 0 "/Game/Chess/Blueprints/ChessPieces/BP_Piece_Child_king.BP_Piece_Child_king_C"))
  (bind _array_element (Utilities|Array|ForEachLoopwithBreak _outactors :!label _label)
    (:LoopBody
      (if (== (Variables|/Game/Chess/Blueprints/ChessPieces/BP_PieceParent.BP_PieceParent_C|GetPieceColor _array_element) Color)
        (LocalVariables|SetdesiredKing _array_element)
        (goto _label Break)))
    (:Completed
      (return (LocalVariables|GetdesiredKing)))))